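; BP_Busch is a physics-driven bush that hops around by itself while the player character is not overlapping it.
; A Startgame event enables physics on PlainBusch and resets the proximity flag, which actor overlaps then toggle.
; While that flag is false, Tick feeds latent Delays that periodically apply an upward and sideways impulse and separately re-roll two random bools choosing its axis and sign.
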(event Custom|Start%20game
  (Variables|Default|SetPlayerIsNahe false)
  (Physics|SetSimulatePhysics (Variables|Default|GetPlain_Busch) true))

(event EventTick
  (params (DeltaSeconds :type Float%20%28single-precision%29))
  (bind _plain_busch (Variables|Default|GetPlain_Busch))
  (if (not (Variables|Default|GetPlayerIsNahe))
    (Utilities|FlowControl|Sequence
      (:then_0
        (Utilities|FlowControl|Delay (Variables|Default|GetTriggertime))
        (if (stale _output_get)
          (Physics|AddImpulse _plain_busch (Math|Vector|MakeVector 0.0 (select (stale _output_get_2) -2.5e+04 2.5e+04) 2.5e+04) "None" false)
          (else
            (Physics|AddImpulse _plain_busch (Math|Vector|MakeVector (select (stale _output_get_2) -2.5e+04 2.5e+04) 0.0 2.5e+04) "None" false))))
      (:then_1
        (Utilities|FlowControl|Delay 1e+01)
        (bind _output_get (Variables|Default|SetRandomInputswitch (Math|Random|RandomBool)))
        (bind _output_get_2 (Variables|Default|SetRandomInputswitch2 (Math|Random|RandomBool)))))))

(event Collision|EventActorBeginOverlap
  (params (OtherActor :type Actor%20Object%20Reference))
  (Utilities|Casting|CastToBP_PlayerCharacter OtherActor)
  (Variables|Default|SetPlayerIsNahe true))

(event Collision|EventActorEndOverlap
  (params (OtherActor :type Actor%20Object%20Reference))
  (Utilities|Casting|CastToBP_PlayerCharacter OtherActor)
  (Variables|Default|SetPlayerIsNahe false))

(fn ConstructionScript)