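; BP_LichtBlockaut_Kronleuchter is a chandelier light Blueprint with four point lights that start switched off.
; The construction script applies intensity, temperature and attenuation radius uniformly to all four lights.
; BeginPlay hides the lights, and the overridden Lichton event calls its parent before making them visible.
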(event EventLichton
  (|CallParentFunction)
  (Rendering|SetVisibility (Variables|Default|GetPointLight1) true false))

(event EventBeginPlay
  (Rendering|SetVisibility (Variables|Default|GetPointLight1) false false))

(fn ConstructionScript
  (bind _pointlight1 (Variables|Default|GetPointLight1))
  (Rendering|Components|Light|SetIntensity (Variables|Default|GetPointLight2) (Variables|Default|GetNew%20Intensity))
  (Class|LightComponent|SetTemperature _pointlight1 (Variables|Default|GetNew%20Temperature))
  (Rendering|Lighting|SetAttenuationRadius _pointlight1 (Variables|Default|GetNew%20Radius)))