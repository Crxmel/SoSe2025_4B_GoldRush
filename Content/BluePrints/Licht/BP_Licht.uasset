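; BP_Licht is a wall lamp Blueprint that starts dark and lights up when its Lichton event fires.
; The construction script applies configurable intensity, temperature and attenuation radius to the PointLight.
; BeginPlay hides the light and creates a dynamic material instance for the lamp glass on the Wandlampe mesh.
; Lichton calls its parent implementation, shows the light and raises the glass's emissive strength.
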(event EventLichton
  (|CallParentFunction)
  (Rendering|SetVisibility (Variables|Default|GetPointLight) true false)
  (Rendering|Material|SetScalarParameterValue (Variables|Default|GetMID) "EmissivStrenght" 1.0 :!class /Script/Engine.MaterialInstanceDynamic))

(event EventBeginPlay
  (Rendering|SetVisibility (Variables|Default|GetPointLight) false false)
  (bind _returnvalue (Rendering|Material|CreateDynamicMaterialInstance (Variables|Default|GetWandlampe) 1 "/Game/Material/Base_Material/MI_Lampenglass.MI_Lampenglass" "None" :!class /Script/Engine.PrimitiveComponent))
  (Variables|Default|SetMID _returnvalue))

(fn ConstructionScript
  (Rendering|Components|Light|SetIntensity (Variables|Default|GetPointLight) (Variables|Default|GetNew%20Intensity))
  (Class|LightComponent|SetTemperature (Variables|Default|GetPointLight) (Variables|Default|GetNew%20Temperature))
  (Rendering|Lighting|SetAttenuationRadius (Variables|Default|GetPointLight) (Variables|Default|GetNew%20Radius)))