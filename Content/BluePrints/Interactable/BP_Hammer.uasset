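; BP_Hammer is an interactable hammer that the player can pick up.
; InteractPickup runs the parent pickup logic, prints a German debug message for pickup or drop, and sets PlayerHasHammer on the character at pickup.
; The drop branch leaves that flag unchanged.
; SetVisibility applies the stored Visebliti bool to the three mesh components, then inverts it, so each call toggles the hammer's visibility.
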(event Custom|SetVisibility
  (Rendering|SetVisibility (Variables|Default|GetCube_0) (Variables|Default|GetVisebliti) false)
  (Variables|Default|SetVisebliti (not (Variables|Default|GetVisebliti))))

(event EventInteractPickup
  (params (PlayerCharacter :type BP%20Player%20Character%20Object%20Reference) (WillPlayerWatchingObjectInHand? :type Boolean) (IsObjectInHand? :type Boolean))
  (|CallParentFunction PlayerCharacter WillPlayerWatchingObjectInHand? IsObjectInHand?)
  (if IsObjectInHand?
    (Development|PrintString "Hammer fallen gelassen")
    (else
      (Development|PrintString "Hammer aufgehoben")
      (Variables|/Game/BluePrints/Character/BP_PlayerCharacter.BP_PlayerCharacter_C|SetPlayerHasHammer? (Variables|Default|GetPlayer%20Character) true))))

(fn ConstructionScript)