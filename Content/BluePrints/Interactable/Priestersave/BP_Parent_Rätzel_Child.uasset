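; Priest's safe interactable, a child of the parent puzzle Blueprint, that opens only when the player holds the priest key.
; With the key, pickup runs the parent logic and a timeline rolls the door open, then returns to the character and loads the level map after a delay.
; Without the key, it shows the safe's UI prompt and calls the interact-block function on the Key.
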(event EventInteractPickup
  (params (PlayerCharacter :type BP%20Player%20Character%20Object%20Reference) (WillPlayerWatchingObjectInHand? :type Boolean) (IsObjectInHand? :type Boolean) (IsPosessesBlockt? :type Boolean))
  (if (Variables|/Game/BluePrints/Character/BP_PlayerCharacter.BP_PlayerCharacter_C|GetHasPlayerPriesterKey? PlayerCharacter)
    (|CallParentFunction PlayerCharacter WillPlayerWatchingObjectInHand? IsObjectInHand? false)
    (bind _rotation (Timeline|DoorOpen PlayFromStart)
      (:Update
        (Transformation|SetRelativeRotation (Variables|Default|GetDoor) (Math|Rotator|MakeRotator (* _rotation 9e+01) 0.0 0.0) false false))
      (:Finished
        (CallFunction|ReturntoCharacter)
        (Utilities|FlowControl|Delay 5.0)
        (Game|OpenLevel(byObjectReference) "/Game/Levels/L_LevelMap.L_LevelMap")))
    (else
      (Default|PriestertresorUI (Variables|/Game/BluePrints/Character/BP_PlayerCharacter.BP_PlayerCharacter_C|GetMainUI PlayerCharacter))
      (Default|InteractBlockBool (Variables|Default|GetKey)))))

(fn ConstructionScript
  (|CallParentFunction))