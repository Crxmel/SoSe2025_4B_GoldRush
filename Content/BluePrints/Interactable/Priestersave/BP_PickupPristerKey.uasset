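; BP_PickupPristerKey is an interactable key pickup, filed under the Priestersave interactables.
; It overrides InteractPickup to run the parent pickup only while InteractBlock is false, then updates button elements on the player's MainUI through TotoButton.
; InteractblockBool toggles that block flag, and the construction script only calls the parent.
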(event Custom|Interact%20block%20Bool
  (Variables|Default|SetInteract%20Block (not (Variables|Default|GetInteract%20Block))))

(event EventInteractPickup
  (params (PlayerCharacter :type BP%20Player%20Character%20Object%20Reference) (WillPlayerWatchingObjectInHand? :type Boolean) (IsObjectInHand? :type Boolean) (IsPosessesBlockt? :type Boolean))
  (if (not (Variables|Default|GetInteract%20Block))
    (|CallParentFunction PlayerCharacter WillPlayerWatchingObjectInHand? IsObjectInHand? IsPosessesBlockt?)
    (Default|TotoButton (Variables|/Game/BluePrints/Character/BP_PlayerCharacter.BP_PlayerCharacter_C|GetMainUI PlayerCharacter) true true false false false false)))

(fn ConstructionScript
  (|CallParentFunction))