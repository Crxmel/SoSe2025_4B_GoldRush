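; BP_Pickup is an interactable physics object that the player can pick up, inspect and drop.
; InteractPickup attaches it to the character's side spot on pickup, registers it as the held object and disables Cube physics.
; When inspection is requested, it toggles between the character's watch and side spots.
; Dropping detaches it, re-enables physics and resets the inspection state.
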(event EventInteractPickup
  (params (PlayerCharacter :type BP%20Player%20Character%20Object%20Reference) (WillPlayerWatchingObjectInHand? :type Boolean) (IsObjectInHand? :type Boolean))
  (if WillPlayerWatchingObjectInHand?
    ;[0.15 0.15 0.15 0.5] Watching object
    (bind _output_get (Variables|Default|SetPlayerWillWatchObject (not (Variables|Default|GetPlayerWillWatchObject))))
    (if _output_get
      (Development|PrintString "Watchspot")
      (Transformation|AttachComponentToComponent (Variables|/Game/BluePrints/Character/BP_PlayerCharacter.BP_PlayerCharacter_C|GetObjectWatchSpot (Variables|Default|GetPlayer%20Character)) "None" "SnapToTarget" "SnapToTarget" "KeepWorld" true)
      (else
        (Development|PrintString "side spot")
        (Transformation|AttachComponentToComponent (Variables|/Game/BluePrints/Character/BP_PlayerCharacter.BP_PlayerCharacter_C|GetObjectSideSpot (Variables|Default|GetPlayer%20Character)) "None" "SnapToTarget" "SnapToTarget" "KeepWorld" true)))
    (else
      (bind _output_get_2 (Variables|Default|SetPlayer%20Character PlayerCharacter))
      (if IsObjectInHand?
        ;[0.15 0.15 0.15 0.5] Object In Hand / Drop
        (Transformation|DetachFromActor "KeepWorld" "KeepWorld" "KeepWorld")
        (Physics|SetSimulatePhysics (Variables|Default|GetCube) true)
        (Variables|Default|SetPlayerWillWatchObject false)
        (else
          (Transformation|AttachComponentToComponent (Variables|/Game/BluePrints/Character/BP_PlayerCharacter.BP_PlayerCharacter_C|GetObjectSideSpot _output_get_2) "None" "SnapToTarget" "SnapToTarget" "KeepWorld" true)
          (Default|ObyectinHand (Variables|Default|GetPlayer%20Character) self)
          (Physics|SetSimulatePhysics (Variables|Default|GetCube) false))))))

(fn ConstructionScript)