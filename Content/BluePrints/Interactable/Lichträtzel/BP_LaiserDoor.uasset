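; Double door for a laser light puzzle that swings open when all four linked lasers report a hit.
; Hit and miss events adjust a counter that plays the rotation Timeline at four and reverses it otherwise.
; A one-time player overlap switches on church-door UI, blends the camera to the door and plays an Actor Sequence cutscene.
; A sequencer event restores view and UI, with a timed delay as backup.
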(event Custom|Laiser%20Hit_Event
  ;[0.15 0.06355 0 0.5] um nicht übers ziel hinaus zu schießen
  (if (> (Variables|Default|GetLaiserOnPoint) -1)
    ;[0.01001 0.15 0 0.5] LaiserRightCounter
    (Variables|Default|SetLaiserOnPoint (+ (Variables|Default|GetLaiserOnPoint) 1))
    (if (== (Variables|Default|GetLaiserOnPoint) 4)
      (bind _output_get (Variables|Default|SetLaiserHitAll true))
      (if _output_get
        ;[0.15 0 0 0.5] Debug
        (if (Variables|Default|GetDebug)
          (Development|PrintString "Door open" true true "(R=0.053815,G=1.000000,B=0.000000,A=1.000000)" 5.0))
        (Utilities|FlowControl|Sequence
          (:then_0
            (Utilities|FlowControl|DelayUntilNextTick)
            (bind (_direction _door_open _griff _time) (Timeline|Timeline Play)
              (:Update
                (Transformation|SetRelativeRotation (Variables|Default|GetRotationpoinl_R) (Math|Rotator|MakeRotator 0.0 0.0 (* _door_open 9e+01)) false false)
                (Transformation|SetRelativeRotation (Variables|Default|GetRotationpoinl_L) (Math|Rotator|MakeRotator 0.0 0.0 (/ (* _door_open 9e+01) -1.0)) false false))
              (:Finished
                (Variables|Default|SetAniTime _time))))
          (:then_1
            (Timeline|Timeline Stop))))
      (else
        (Variables|Default|SetLaiserHitAll false)
        ;[0.15 0 0.003522 0.5] Debug
        (if (Variables|Default|GetDebug)
          (Development|PrintString (Utilities|String|Append "Laiser right :     " (Utilities|String|ToString(Integer) (Variables|Default|GetLaiserOnPoint))) true true "(R=0.044389,G=1.000000,B=0.000000,A=1.000000)" 5.0))
        (Utilities|FlowControl|Sequence
          (:then_0
            (Timeline|Timeline Stop))
          (:then_1
            (Utilities|FlowControl|DelayUntilNextTick)
            (Timeline|Timeline Reverse)))))))

(event Custom|Laiser%20Dont%20Hit_Event
  ;[0.15 0.06355 0 0.5] um nicht übers ziel hinaus zu schießen
  (if (< (Variables|Default|GetLaiserOnPoint) 5)
    ;[0.01001 0.15 0 0.5] LaiserRightCounter
    (Variables|Default|SetLaiserOnPoint (- (Variables|Default|GetLaiserOnPoint) 1))
    (if (== (Variables|Default|GetLaiserOnPoint) 4)
      (bind _output_get (Variables|Default|SetLaiserHitAll true))
      (if _output_get
        ;[0.15 0 0 0.5] Debug
        (if (Variables|Default|GetDebug)
          (Development|PrintString "Door open" true true "(R=0.053815,G=1.000000,B=0.000000,A=1.000000)" 5.0))
        (Utilities|FlowControl|Sequence
          (:then_0
            (Utilities|FlowControl|DelayUntilNextTick)
            (bind (_direction _door_open _griff _time) (Timeline|Timeline Play)
              (:Update
                (Transformation|SetRelativeRotation (Variables|Default|GetRotationpoinl_R) (Math|Rotator|MakeRotator 0.0 0.0 (* _door_open 9e+01)) false false)
                (Transformation|SetRelativeRotation (Variables|Default|GetRotationpoinl_L) (Math|Rotator|MakeRotator 0.0 0.0 (/ (* _door_open 9e+01) -1.0)) false false))
              (:Finished
                (Variables|Default|SetAniTime _time))))
          (:then_1
            (Timeline|Timeline Stop))))
      (else
        (Variables|Default|SetLaiserHitAll false)
        ;[0.15 0 0.003522 0.5] Debug
        (if (Variables|Default|GetDebug)
          (Development|PrintString (Utilities|String|Append "Laiser right :     " (Utilities|String|ToString(Integer) (Variables|Default|GetLaiserOnPoint))) true true "(R=0.044389,G=1.000000,B=0.000000,A=1.000000)" 5.0))
        (Utilities|FlowControl|Sequence
          (:then_0
            (Timeline|Timeline Stop))
          (:then_1
            (Utilities|FlowControl|DelayUntilNextTick)
            (Timeline|Timeline Reverse)))))))

(event Custom|CutscreenEnde
  (params (is%20triggert :type Boolean))
  ;[0.15 0.15 0.15 0.5] Cutsceene triger und Ui an/aus
  (Default|Kirchentür (Variables|/Game/BluePrints/Character/BP_PlayerCharacter.BP_PlayerCharacter_C|GetMainUI (Variables|Default|GetPlayer%20Character)) false)
  (Game|Player|SetViewTargetwithBlend (Game|GetPlayerController 0) (Variables|Default|GetPlayer%20Character) 1.5 "VTBlend_EaseInOut" 1.5 false))

(event Custom|Player%20exit)

(event EventBeginPlay
  (EventDispatchers|AssignLaiserHit (Variables|Default|GetLaiser_01) (delegate Custom|Laiser%20Hit_Event))
  (EventDispatchers|AssignLaiserDontHit (Variables|Default|GetLaiser_01) (delegate Custom|Laiser%20Dont%20Hit_Event))
  (Rendering|SetVisibility (Variables|Default|GetZielhöhe) false false))

(event Collision|EventActorBeginOverlap
  (params (OtherActor :type Actor%20Object%20Reference))
  ;[0.15 0.15 0.15 0.5] Cutsceene triger und Ui an/aus
  (Utilities|FlowControl|DoOnce (Variables|Default|GetLaiserHitAll)
    (:Completed
      (bind _asbp_player_character (Utilities|Casting|CastToBP_PlayerCharacter OtherActor))
      (bind _output_get (Variables|Default|SetPlayer%20Character _asbp_player_character))
      (Default|Kirchentür (Variables|/Game/BluePrints/Character/BP_PlayerCharacter.BP_PlayerCharacter_C|GetMainUI _output_get) true)
      (Game|Player|SetViewTargetwithBlend (Game|GetPlayerController 0) self 1.5 "VTBlend_EaseInOut" 1.5 false)
      (Class|ActorSequenceComponent|PlaySequence (Variables|Default|GetActorSequence))
      (Utilities|FlowControl|Delay 7.0)
      (if (stale Custom|CutscreenEnde is%20triggert)
        (Development|PrintString "Bagsicherrung nicht nötig" true true "(R=0.198435,G=1.000000,B=0.000000,A=1.000000)" 5.0)
        (else
          (Development|PrintString "Bagsicherrung nötig" true true "(R=1.000000,G=0.067559,B=0.000000,A=1.000000)" 5.0)
          (Default|Kirchentür (Variables|/Game/BluePrints/Character/BP_PlayerCharacter.BP_PlayerCharacter_C|GetMainUI (Variables|Default|GetPlayer%20Character)) false)
          (Game|Player|SetViewTargetwithBlend (Game|GetPlayerController 0) (Variables|Default|GetPlayer%20Character) 1.5 "VTBlend_EaseInOut" 1.5 false))))))

(event Custom|BP_LaiserDoor0_Event
  (params (BP_LaiserDoor0 :type Actor%20Object%20Reference))
  (CallFunction|CutscreenEnde true))

(fn ConstructionScript)