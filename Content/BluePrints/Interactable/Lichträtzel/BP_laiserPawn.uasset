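; Interactable light-puzzle laser pawn that acts as a beam source or redirector, which the player rotates by yaw input until exiting.
; Sources line-trace every tick, size the Niagara beam to the hit and notify BP_laiserEbpfang receivers.
; Pawns hit on their Box relay the beam recursively when allowed, copying the gameplay tag and using game-time checks to switch off.
; Possession is gated on generator state, but the generator event binding never runs.
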(event Custom|GetHitByLaiser
  (params (A :type Object%20Object%20Reference) (Laisersource :type BP%20Laiser%20Pawn%20Object%20Reference))
  ;[0.15 0.15 0.15 0.5] Laiser weiterleiten
  (if (== A (Variables|Default|GetBox))
    (if (CallFunction|TimeHasPassedSinceLastHit)
      (Variables|Default|SetLastHitTime (Utilities|Time|GetGameTimeinSeconds))
      (if (Variables|Default|GetCanReaderectLight)
        (GameplayTags|AddGameplayTag (Variables|/Game/BluePrints/Interactable/BP_Tags.BP_Tags_C|GetTagContain (Variables|Default|GetBP_Tags)) (Variables|BP_laiserPawn_C|GetTag Laisersource) :!class /Script/GameplayTags.BlueprintGameplayTagLibrary)
        (CallFunction|SetVFXEnabled true)
        (bind (_stop_lin _returnvalue) (CallFunction|EmitLaiser))
        (CallFunction|LaiserHitZiel _stop_lin _returnvalue)))))

(event Custom|LaiserHitZiel
  (params (HitLaiser :type Boolean) (EmpfangActor :type Object%20Object%20Reference))
  ;[0.009562 0.15 0 0.5] FürLaiserZiel
  (if HitLaiser
    (Utilities|FlowControl|Sequence
      (:then_0
        (Utilities|FlowControl|DoOnce false :!label _label
          (:Completed
            _)))
      (:then_1
        (goto _label_2 Reset)))
    (else
      (Utilities|FlowControl|Sequence
        (:then_0
          (goto _label Reset))
        (:then_1
          (Utilities|FlowControl|DoOnce false :!label _label_2
            (:Completed
              _))))))
  (Variables|Default|SetHitLaiser (not HitLaiser))
  (bind _asbp_laiser_ebpfang (Utilities|Casting|CastToBP_laiserEbpfang EmpfangActor)
    (:then
      (bind _output_get (Variables|Default|SetAs%20BP%20Laiser%20Ebpfang _asbp_laiser_ebpfang))
      (Utilities|IsValid _output_get :!label _label_3
        (:Is%20Valid
          (Default|LaiserDings _output_get (Variables|Default|GetHitLaiser) self (Variables|Default|GetPlayer%20CHaracter)))))
    (:CastFailed
      (Utilities|FlowControl|Sequence
        (:then_0
          (goto _label_3))
        (:then_1
          (Utilities|FlowControl|DelayUntilNextTick)
          (Variables|Default|SetAs%20BP%20Laiser%20Ebpfang 0))))))

(event Custom|GenAn_Event
  (Variables|Default|SetIsGenOn true)
  (CallFunction|SetVFXEnabled (Variables|Default|GetIsLaiserSource)))

(event Input|EnhancedActionEvents|EnhancedInputActionIA_PuzzleMous
  (params (ActionValue :type Vector%202D%20Structure) (ElapsedSeconds :type Float%20%28double-precision%29) (TriggeredSeconds :type Float%20%28double-precision%29) (InputAction :type Input%20Action%20Object%20Reference :default "/Game/Input/Rätzel/IA_PuzzleMous.IA_PuzzleMous"))
  ;[0.15 0.1348 0 0.5] Navigate
  (Transformation|AddLocalRotation (Variables|Default|GetRotationPoint) (Math|Rotator|MakeRotator 0.0 0.0 (* (.x ActionValue) (Utilities|Time|GetWorldDeltaSeconds) (Variables|Default|GetRotationspeed))) false false))

(event Input|EnhancedActionEvents|EnhancedInputActionIA_PuzzleExit
  (params (ActionValue :type Boolean) (ElapsedSeconds :type Float%20%28double-precision%29) (TriggeredSeconds :type Float%20%28double-precision%29) (InputAction :type Input%20Action%20Object%20Reference :default "/Game/Input/Rätzel/IA_PuzzleExit.IA_PuzzleExit"))
  ;[0.15 0.1348 0 0.5] Navigate
  (CallFunction|ReturntoCharacter)
  (Default|PlayerExit (Variables|Default|GetBP_LaiserDoor_ZmÖffnen))
  (Default|TotoButton (Variables|/Game/BluePrints/Character/BP_PlayerCharacter.BP_PlayerCharacter_C|GetMainUI (Variables|Default|GetPlayer%20CHaracter)) false false false false false false))

(event EventBeginPlay
  (bind _tag (Variables|Default|GetTag))
  (Components|Activation|Deactivate (Variables|Default|GetNS_Beam))
  (if (Variables|Default|GetIsLaiserSource)
    (GameplayTags|AddGameplayTag (Variables|/Game/BluePrints/Interactable/BP_Tags.BP_Tags_C|GetTagContain (Variables|Default|GetBP_Tags)) _tag :!class /Script/GameplayTags.BlueprintGameplayTagLibrary)
    ;[0.15 0 0 0.5] Debug
    (if (Variables|Default|GetDebug)
      (Development|PrintString (Utilities|String|Append "ADD GamePlayTag" (Utilities|String|ToString(Name) (GameplayTags|GetTagName _tag))) true true "(R=0.025951,G=1.000000,B=0.000000,A=1.000000)" 5.0))))

(event EventInteractPickup
  (params (PlayerCharacter :type BP%20Player%20Character%20Object%20Reference) (WillPlayerWatchingObjectInHand? :type Boolean) (IsObjectInHand? :type Boolean) (IsPosessesBlockt? :type Boolean))
  (|CallParentFunction PlayerCharacter WillPlayerWatchingObjectInHand? IsObjectInHand? (not (Variables|Default|GetIsGenOn)))
  (Default|TotoButton (Variables|/Game/BluePrints/Character/BP_PlayerCharacter.BP_PlayerCharacter_C|GetMainUI (Variables|Default|GetPlayer%20CHaracter)) true false false true false false))

(event EventTick
  (params (DeltaSeconds :type Float%20%28single-precision%29))
  ;[0.15 0.15 0.15 0.5] Laiser Start
  (if (Variables|Default|GetIsLaiserSource)
    (bind (_stop_lin _returnvalue) (CallFunction|EmitLaiser))
    (CallFunction|LaiserHitZiel _stop_lin _returnvalue)
    (elif (CallFunction|TimeHasPassedSinceLastHit)
      (CallFunction|SetVFXEnabled false))))

(fn ConstructionScript
  (|CallParentFunction)
  (Transformation|AddLocalRotation (Variables|Default|GetRotationPoint) (.rotation (Variables|Default|GetStartRotation)) false false))

(fn SetVFXEnabled
  (params (IsEnabled :type Boolean))
  (bind _ns_beam (Variables|Default|GetNS_Beam))
  (if IsEnabled
    (Components|Activation|Activate _ns_beam false)
    (else
      (Components|Activation|Deactivate _ns_beam))))

(fn CheckforLaisetHit
  (bind _laiser_origen (Variables|Default|GetLaiser%20origen))
  (bind _returnvalue (Transformation|GetWorldLocation _laiser_origen))
  (bind (_outhit _returnvalue_2) (Collision|LineTraceForObjects _returnvalue (+ _returnvalue (* (Math|Vector|GetForwardVector _laiser_origen) (Variables|Default|GetMaxLaiserRange))) (Utilities|Array|MakeArray "ObjectTypeQuery1" "ObjectTypeQuery2" "ObjectTypeQuery3" "ObjectTypeQuery4") false 0 (select (Variables|Default|GetDebug) "ForOneFrame" "None")))
  (if _returnvalue_2
    (bind _asbp_laiser_pawn (Utilities|Casting|CastToBP_laiserPawn (.HitActor (Collision|BreakHitResult _outhit)))
      (:then
        _)
      (:CastFailed
        _))
    (return true (Math|Vector|VectorLength (- (.ImpactPoint (Collision|BreakHitResult _outhit)) (Transformation|GetWorldLocation (Variables|Default|GetLaiser%20origen)))) _asbp_laiser_pawn (.HitComponent (Collision|BreakHitResult _outhit)))
    (else
      (return false 0.0 0 0))))

(fn EmitLaiser
  (bind (_hitsomphing _distancetohit _asbp_laiser_pawn _hitcomponent) (CallFunction|CheckforLaisetHit))
  (if _hitsomphing
    (Niagara|SetNiagaraVariable(Float) (Variables|Default|GetNS_Beam) "LaiserLenght" _distancetohit)
    (Utilities|IsValid _asbp_laiser_pawn
      (:Is%20Valid
        (CallFunction|GetHitbyLaiser _asbp_laiser_pawn _hitcomponent self)
        (return true 0))
      (:Is%20Not%20Valid
        (bind _asbp_laiser_ebpfang (Utilities|Casting|CastToBP_laiserEbpfang (Components|GetOwner _hitcomponent))
          (:then
            (return false _asbp_laiser_ebpfang))
          (:CastFailed
            (return true 0)))))
    (else
      (return true 0))))

(fn TimeHasPassedSinceLastHit
  (return (> (Utilities|Time|GetGameTimeinSeconds) (Variables|Default|GetLastHitTime))))