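; Laser receiver for the interactable light puzzle that reports whether a laser from a matching source is hitting it.
; The LaiserDings event stores the hit state and checks the source's BP_Tags component for an exact match with TagToNeed.
; Matching sources trigger the LaiserHit or LaiserDontHit call depending on that state, while other sources trigger neither.
; A Debug flag prints the hit state and tag result.
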(event Custom|LaiserDings
  (params (HitLaiser :type Boolean) (LaiserSource :type BP%20Laiser%20Pawn%20Object%20Reference) (PlayerCharakter :type BP%20Player%20Character%20Object%20Reference))
  (bind _returnvalue (Actor|GetComponentbyClass LaiserSource "/Game/BluePrints/Interactable/BP_Tags.BP_Tags_C"))
  (bind _tagtoneed (Variables|Default|GetTagToNeed))
  (bind _tagcontain (Variables|/Game/BluePrints/Interactable/BP_Tags.BP_Tags_C|GetTagContain _returnvalue))
  (bind _returnvalue_2 (GameplayTags|HasTag _tagcontain _tagtoneed true))
  (bind _output_get (Variables|Default|SetLaiserHit HitLaiser))
  ;[0.15 0 0 0.5] Debug
  (if (Variables|Default|GetDebug)
    (Development|PrintString (Utilities|String|Append "LaiserHit:__" (Utilities|String|ToString(Boolean) _output_get)) true true "(R=0.421148,G=1.000000,B=0.423622,A=1.000000)" 5.0))
  (Utilities|IsValid _returnvalue
    (:Is%20Valid
      ;[0.15 0 0 0.5] Debug
      (if (Variables|Default|GetDebug)
        (Development|PrintString (Utilities|String|Append "Tag   " (Utilities|String|ToString(Boolean) _returnvalue_2)) true true "(R=0.397902,G=1.000000,B=0.470820,A=1.000000)" 5.0))
      (if _returnvalue_2
        (if (Variables|Default|GetLaiserHit)
          (Default|CallLaiserHit)
          (else
            (Default|CallLaiserDontHit)))))))

(fn ConstructionScript)