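; BP_Latte1 is an interactable wooden slat ("Latte") that gets knocked loose by an animated hammer when the player interacts with it.
; InteractPickup runs once, calls the parent, shows the built-in Hammer and waits out SmoothProsessDuration.
; Parallel timelines then swing the hammer and, slightly delayed, fling Cube01 away before destroying it and tilt FallendeLatte.
; Afterwards it destroys the Hammer, calls ReturnToCharacter and calls SetVisibility on the player's held BP_Hammer.
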(event EventInteractPickup
  (params (PlayerCharacter :type BP%20Player%20Character%20Object%20Reference) (WillPlayerWatchingObjectInHand? :type Boolean) (IsObjectInHand? :type Boolean))
  (bind _hammer (Variables|Default|GetHammer))
  (bind _cube_0_1 (Variables|Default|GetCube_0_1))
  (Utilities|FlowControl|DoOnce false
    (:Completed
      (|CallParentFunction PlayerCharacter WillPlayerWatchingObjectInHand? IsObjectInHand?)
      (Rendering|SetVisibility (Variables|Default|GetHammer) true false)
      (Utilities|FlowControl|Delay (Variables|Default|GetSmooth%20Prosess%20Duration))
      (Utilities|FlowControl|Sequence
        (:then_1
          (bind (_direction _bewegung _bewegung_höhe _rotation) (Timeline|Hammer_Animation PlayFromStart)
            (:Update
              (Transformation|SetRelativeLocation _hammer (Math|Vector|MakeVector (* _bewegung 8e+01) 0.0 (* _bewegung_höhe -8e+01)) false false)
              (Transformation|SetRelativeRotation _hammer (Math|Rotator|MakeRotator 0.0 (* _rotation -1.2e+02) 0.0) false false))
            (:Finished
              (Utilities|FlowControl|Delay 0.6)
              (Components|DestroyComponent (Variables|Default|GetHammer))
              (CallFunction|ReturntoCharacter)
              (bind _asbp_hammer (Utilities|Casting|CastToBP_Hammer (Variables|/Game/BluePrints/Character/BP_PlayerCharacter.BP_PlayerCharacter_C|GetObyect%20in%20Hand (Variables|Default|GetPlayer%20CHaracter))))
              (Default|SetVisibility _asbp_hammer))))
        (:then_2
          (Utilities|FlowControl|Delay 0.8)
          (bind _lattenwegfliegen (Timeline|WegfliegbrettTimeline PlayFromStart)
            (:Update
              (Transformation|SetRelativeLocation _cube_0_1 (Math|Vector|MakeVector 0.0 (* _lattenwegfliegen 5e+02) (* _lattenwegfliegen 3e+02)) false false)
              (Transformation|SetRelativeRotation _cube_0_1 (Math|Rotator|MakeRotator (* _lattenwegfliegen 6.5e+02) 0.0 0.0) false false))
            (:Finished
              (Components|DestroyComponent _cube_0_1))))
        (:then_3
          (Utilities|FlowControl|Delay 0.8)
          (bind _newtrack_0 (Timeline|WegfallBrett PlayFromStart)
            (:Update
              (Transformation|SetRelativeRotation (Variables|Default|GetFallende%20latte) (Math|Rotator|MakeRotator (* _newtrack_0 45.0) 0.0 0.0) false false))))))))

(fn ConstructionScript)