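; Castle door with a lockpick (Dietrich) puzzle, playable only when the player carries a pick.
; Confirming the UI prompt calls the parent's GetProsses to hand control to the door, where mouse input rolls the pick.
; BeginPlay randomizes target angle and tolerance, and Tick triggers a wiggle timeline inside that range.
; The action input plays a jiggle; a correct angle returns control, removes the pick and swings the door open.
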(event Custom|DietrichPuzzleFinish
  ;[0.15 0.15 0.15 0.5] Dietrich UI De/Aktiviren
  (CallFunction|ReturntoCharacter)
  (Rendering|SetVisibility (Variables|Default|GetRätzeldietrich) false false)
  (Default|TotoButton (Variables|/Game/BluePrints/Character/BP_PlayerCharacter.BP_PlayerCharacter_C|GetMainUI (stale EventInteractPickup PlayerCharacter)) false false false false false false false))

(event Custom|LösungSetByBeginPlay
  ;[0.01535 0.15 0 0.5] Custom Lösung erstellen
  (bind _output_get (Variables|Default|SetSpannweite (Math|Random|RandomIntegerinRange 12 20)))
  (if (Variables|Default|GetDebug)
    ;;[0.15 0 0 0.5] debug mode
    (Development|PrintString (Utilities|String|Append (Utilities|String|ToString(Integer) _output_get) " : " (Utilities|GetDisplayName self)) true true "(R=0.000000,G=0.660000,B=1.000000,A=1.000000)" 1e+08))
  (bind _output_get_2 (Variables|Default|SetLösungswert (Math|Random|RandomIntegerinRange -165 165)))
  (if (Variables|Default|GetDebug)
    (Development|PrintString (Utilities|String|Append (Utilities|String|ToString(Integer) _output_get_2) " : " (Utilities|GetDisplayName self)) true true "(R=0.302297,G=1.000000,B=0.430968,A=1.000000)" 1e+11)))

(event Custom|ButtonDietrichWirdBenutzt
  ;[0.15 0.15 0.15 0.5] totorial UI De/Aktiviren
  (if (Variables|Default|GetHasInteract)
    (CallFunction|GetProsses (stale EventInteractPickup PlayerCharacter) self)
    (Variables|Default|SetHasInteract false)
    ;[0.15 0.15 0.15 0.5] Dietrich UI De/Aktiviren
    (if (not (Variables|Default|GetIs%20Posesses%20Blockt?))
      (Rendering|SetVisibility (Variables|Default|GetRätzeldietrich) true false))))

(event Input|EnhancedActionEvents|EnhancedInputActionIA_PuzzleExit
  (params (ActionValue :type Boolean) (ElapsedSeconds :type Float%20%28double-precision%29) (TriggeredSeconds :type Float%20%28double-precision%29) (InputAction :type Input%20Action%20Object%20Reference :default "/Game/Input/Rätzel/IA_PuzzleExit.IA_PuzzleExit"))
  ;[0.15 0.15 0.15 0.5] Dietrich UI De/Aktiviren
  (CallFunction|ReturntoCharacter)
  (Rendering|SetVisibility (Variables|Default|GetRätzeldietrich) false false)
  (Default|TotoButton (Variables|/Game/BluePrints/Character/BP_PlayerCharacter.BP_PlayerCharacter_C|GetMainUI (stale EventInteractPickup PlayerCharacter)) false false false false false false false))

(event Input|EnhancedActionEvents|EnhancedInputActionIA_PuzzleMous
  (params (ActionValue :type Vector%202D%20Structure) (ElapsedSeconds :type Float%20%28double-precision%29) (TriggeredSeconds :type Float%20%28double-precision%29) (InputAction :type Input%20Action%20Object%20Reference :default "/Game/Input/Rätzel/IA_PuzzleMous.IA_PuzzleMous"))
  ;[0.15 0.15 0.15 0.5] Rotation Dietrich
  (if (not (Variables|Default|GetISInteractAniPlaying))
    (Transformation|AddRelativeRotation (Variables|Default|GetRotationPoint_Dietrich) (Math|Rotator|MakeRotator (.x ActionValue) 0.0 0.0) false false)))

(event Input|EnhancedActionEvents|EnhancedInputActionIA_PuzzleAction
  (params (ActionValue :type Boolean) (ElapsedSeconds :type Float%20%28double-precision%29) (TriggeredSeconds :type Float%20%28double-precision%29) (InputAction :type Input%20Action%20Object%20Reference :default "/Game/Input/Rätzel/IA_PuzzleAction.IA_PuzzleAction"))
  (bind _rotationpoint_dietrich (Variables|Default|GetRotationPoint_Dietrich))
  (bind _returnvalue (Transformation|GetWorldRotation _rotationpoint_dietrich))
  ;[0.15 0.15 0.15 0.5] Interact
  (Utilities|FlowControl|DoOnce false :!label _label
    (:Completed
      (Utilities|FlowControl|Sequence
        (:then_0
          ;[0.15 0.15 0.15 0.5] input block
          (Variables|Default|SetISInteractAniPlaying true)
          ;;[0.15 0.15 0.15 0.5] Animation bei falschen interact
          (Audio|Components|Audio|Play (Variables|Default|Getfoley-key-key-ring-small-place-02) 0.0)
          (bind _newtrack_0 (Timeline|InteractAni PlayFromStart)
            (:Update
              (Transformation|AddRelativeRotation (Variables|Default|GetRätzeldietrich) (Math|Rotator|MakeRotator (* _newtrack_0 0.6) 0.0 0.0) false false))
            (:Finished
              (Variables|Default|SetISInteractAniPlaying false)
              (goto _label Reset))))
        (:then_1
          (if (and (> (.roll _returnvalue) (- (Variables|Default|GetLösungswert) (/ (Variables|Default|GetSpannweite) 2))) (< (.roll _returnvalue) (+ (Variables|Default|GetLösungswert) (/ (Variables|Default|GetSpannweite) 2))))
            (Utilities|FlowControl|Sequence
              (:then_0
                (Timeline|InteractAni Stop))
              (:then_1
                (CallFunction|DietrichPuzzleFinish)
                (Audio|Components|Audio|Play (Variables|Default|GetSC_Holzdoor) 0.0)
                (Components|DestroyComponent (Variables|Default|GetRätzeldietrich))
                (Utilities|FlowControl|Delay (/ (Variables|Default|GetSmooth%20Prosess%20Duration) 2.0))
                (Default|Has/DonthasDietrich (Variables|Default|GetPlayer%20CHaracter))
                (bind (_direction _door_open _griff) (Timeline|Finige%20ani Play)
                  (:Update
                    (Transformation|SetRelativeRotation (Variables|Default|GetDoor) (Math|Rotator|MakeRotator 0.0 0.0 (* (Variables|Default|GetOpenWinkel) _door_open)) false false)
                    (Transformation|SetRelativeRotation (Variables|Default|GetTürGriff) (Math|Rotator|MakeRotator (* _griff 45.0) 0.0 0.0) false false)))))))))))

(event EventInteractPickup
  (params (PlayerCharacter :type BP%20Player%20Character%20Object%20Reference) (WillPlayerWatchingObjectInHand? :type Boolean) (IsObjectInHand? :type Boolean) (IsPosessesBlockt? :type Boolean))
  (bind _mainui (Variables|/Game/BluePrints/Character/BP_PlayerCharacter.BP_PlayerCharacter_C|GetMainUI PlayerCharacter))
  (Variables|Default|SetHasInteract true)
  ;[0.15 0.15 0.15 0.5] totorial UI De/Aktiviren
  (if (Variables|/Game/BluePrints/Character/BP_PlayerCharacter.BP_PlayerCharacter_C|GetPlayerHasDietrich? PlayerCharacter)
    (Default|DietrichUIRätzelStarten? _mainui)
    (EventDispatchers|BindEventtoButtonDietrichwirdBenutzt _mainui (delegate Custom|ButtonDietrichWirdBenutzt))
    (else
      ;;[0.15 0.15 0.15 0.5] Kein dietrich UI trigger
      (Default|DietrichDoorInteractOhneDietrichUI (Variables|/Game/BluePrints/Character/BP_PlayerCharacter.BP_PlayerCharacter_C|GetMainUI PlayerCharacter))
      (Variables|Default|SetHasInteract true))))

(event EventBeginPlay
  (CallFunction|LösungSetbyBeginPlay))

(event EventReturntoCharacter
  (|CallParentFunction)
  (Variables|Default|SetHasInteract false)
  (Rendering|SetVisibility (Variables|Default|GetRätzeldietrich) false false))

(event EventTick
  (params (DeltaSeconds :type Float%20%28single-precision%29))
  (bind _rotationpoint_dietrich (Variables|Default|GetRotationPoint_Dietrich))
  (bind _returnvalue (Transformation|GetWorldRotation _rotationpoint_dietrich))
  ;[0.15 0.15 0.15 0.5] ditrichAnimation
  (if (and (> (.roll _returnvalue) (- (Variables|Default|GetLösungswert) (/ (Variables|Default|GetSpannweite) 2))) (< (.roll _returnvalue) (+ (Variables|Default|GetLösungswert) (/ (Variables|Default|GetSpannweite) 2))))
    (Utilities|FlowControl|DoOnce false :!label _label
      (:Completed
        (Utilities|FlowControl|Sequence
          (:then_0
            (bind _newtrack_0 (Timeline|Timeline Play)
              (:Update
                (Transformation|AddRelativeRotation (Variables|Default|GetRotationPoint_Dietrich) (Math|Rotator|MakeRotator _newtrack_0 0.0 0.0) false false))))
          (:then_1
            (goto _label_2 Reset)))))
    (else
      (Utilities|FlowControl|DoOnce false :!label _label_2
        (:Completed
          (Utilities|FlowControl|Sequence
            (:then_0
              (goto _label Reset))
            (:then_1
              (Timeline|Timeline Stop))))))))

(fn ConstructionScript
  (|CallParentFunction))