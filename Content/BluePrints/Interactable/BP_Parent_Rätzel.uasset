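; BP_Parent_Rätzel is a parent for interactable puzzles that the player temporarily possesses.
; Interacting, unless possession is blocked, blends the view to the puzzle, possesses it and swaps the Enhanced Input mapping context.
; ReturntoCharacter reverses this after moving the character to the Respawnpoint or the child's camera, grounded by a downward trace.
; Children must supply a CameraComponent, otherwise repositioning only prints an error.
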(event Custom|GetProsses
  (bind _returnvalue (Game|GetPlayerController 0))
  (bind _returnvalue_2 (PlayerController|LocalPlayerSubsystems|GetEnhancedInputLocalPlayerSubsystem _returnvalue))
  (Input|RemoveMappingContext _returnvalue_2 "/Game/Input/Player/IMC_Player.IMC_Player" "(bIgnoreAllPressedKeysUntilRelease=True,bForceImmediately=False,bNotifyUserSettings=False)")
  (Game|Player|SetViewTargetwithBlend (Game|GetPlayerController 0) self (Variables|Default|GetSmooth%20Prosess%20Duration) (Variables|Default|GetBlend%20Func) (Variables|Default|GetSmoothPossessBlendExp) false)
  (Utilities|FlowControl|Delay (Variables|Default|GetSmooth%20Prosess%20Duration))
  (Pawn|Possess (Game|GetPlayerController 0) self)
  (Input|AddMappingContext _returnvalue_2 "/Game/Input/Rätzel/IMC_Rätzel.IMC_Rätzel" 0 "(bIgnoreAllPressedKeysUntilRelease=True,bForceImmediately=False,bNotifyUserSettings=False)"))

(event Custom|Return%20to%20Character
  (bind _returnvalue (Game|GetPlayerController 0))
  (bind _returnvalue_2 (PlayerController|LocalPlayerSubsystems|GetEnhancedInputLocalPlayerSubsystem _returnvalue))
  (CallFunction|PositionPlayerCharacter)
  (Input|RemoveMappingContext _returnvalue_2 "/Game/Input/Rätzel/IMC_Rätzel.IMC_Rätzel" "(bIgnoreAllPressedKeysUntilRelease=True,bForceImmediately=False,bNotifyUserSettings=False)")
  (Game|Player|SetViewTargetwithBlend (Game|GetPlayerController 0) (Variables|Default|GetPlayer%20CHaracter) (Variables|Default|GetSmooth%20Prosess%20Duration) (Variables|Default|GetBlend%20Func) (Variables|Default|GetSmoothPossessBlendExp) false)
  (Utilities|FlowControl|Delay (Variables|Default|GetSmooth%20Prosess%20Duration))
  (Pawn|Possess (Game|GetPlayerController 0) (Variables|Default|GetPlayer%20CHaracter))
  (Input|AddMappingContext _returnvalue_2 "/Game/Input/Player/IMC_Player.IMC_Player" 0 "(bIgnoreAllPressedKeysUntilRelease=True,bForceImmediately=False,bNotifyUserSettings=False)"))

(event EventInteractPickup
  (params (PlayerCharacter :type BP%20Player%20Character%20Object%20Reference) (WillPlayerWatchingObjectInHand? :type Boolean) (IsObjectInHand? :type Boolean) (IsPosessesBlockt? :type Boolean))
  (bind _output_get (Variables|Default|SetPlayer%20CHaracter PlayerCharacter))
  (if (not IsPosessesBlockt?)
    (CallFunction|GetProsses)))

(fn ConstructionScript
  (Rendering|SetVisibility (Variables|Default|GetArrow_8B58CFAD) (Variables|Variable_ParentRätzel|GetDebug) false)
  (Transformation|SetRelativeLocation (Variables|Default|GetRespawnpoint) (.location (Variables|Variable_ParentRätzel|GetSetRespawnpoint)) false false))

(fn PositionPlayerCharacter
  (bind _output_get (LocalVariables|SetCam (Actor|GetComponentbyClass "/Script/Engine.CameraComponent")))
  (Utilities|IsValid _output_get
    (:Is%20Valid
      (Transformation|SetActorLocation (Variables|Default|GetPlayer%20CHaracter) (Transformation|GetWorldLocation (select (Variables|Variable_ParentRätzel|GetSpawnOnRespawnpoint) (Variables|Default|GetRespawnpoint) (LocalVariables|GetCam))) false false)
      (bind (_outhit _returnvalue) (Collision|LineTraceForObjects (Transformation|GetWorldLocation (select (Variables|Variable_ParentRätzel|GetSpawnOnRespawnpoint) (Variables|Default|GetRespawnpoint) (LocalVariables|GetCam))) (- (Transformation|GetWorldLocation (select (Variables|Variable_ParentRätzel|GetSpawnOnRespawnpoint) (Variables|Default|GetRespawnpoint) (LocalVariables|GetCam))) "0.000000,0.000000,300.000000") (Utilities|Array|MakeArray "ObjectTypeQuery1" "ObjectTypeQuery2") false 0 "ForDuration" true "(R=1.000000,G=0.000000,B=0.000000,A=1.000000)" "(R=0.000000,G=1.000000,B=0.000000,A=1.000000)" 1e+01))
      (if _returnvalue
        (Transformation|SetActorLocation (Variables|Default|GetPlayer%20CHaracter) (+ (.Location (Collision|BreakHitResult _outhit)) (Math|Vector|MakeVector 0.0 0.0 (+ (Variables|/Script/Engine.CapsuleComponent|GetCapsuleHalfHeight (Variables|/Script/Engine.Character|GetCapsuleComponent (Variables|Default|GetPlayer%20CHaracter))) 1.0))) false false)))
    (:Is%20Not%20Valid
      (Development|PrintString "BP_InteractableProssessable child braucht cameracomponent konnte aber nix finden" true true "(R=0.000000,G=0.660000,B=1.000000,A=1.000000)" 5.0))))