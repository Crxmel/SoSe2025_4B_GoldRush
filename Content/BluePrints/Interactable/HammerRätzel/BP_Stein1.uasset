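; BP_Stein1 is a hammer-puzzle stone that breaks once when the player interacts with it.
; After the parent pickup logic, a timeline swings the stone's own Hammer component, then the collider is destroyed.
; The hammer is removed, control returns to the character and the held BP_Hammer's visibility is set.
; Meanwhile, the block launches with a physics impulse, scales via timeline, then destroys ActorDestroy and itself.
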(event EventInteractPickup
  (params (PlayerCharacter :type BP%20Player%20Character%20Object%20Reference) (WillPlayerWatchingObjectInHand? :type Boolean) (IsObjectInHand? :type Boolean) (IsPosessesBlockt? :type Boolean))
  (bind _actor_destroy (Variables|Default|GetActor%20destroy))
  (bind _gc_1_skulptet_block2 (Variables|Default|GetGC_1_Skulptet_Block2))
  (bind _hammer (Variables|Default|GetHammer))
  (Utilities|FlowControl|DoOnce false
    (:Completed
      (|CallParentFunction PlayerCharacter WillPlayerWatchingObjectInHand? IsObjectInHand? false)
      (Rendering|SetVisibility (Variables|Default|GetHammer) true false)
      (Utilities|FlowControl|Delay (Variables|Default|GetSmooth%20Prosess%20Duration))
      (bind (_direction _bewegung _bewegung_höhe _rotation) (Timeline|Timeline PlayFromStart)
        (:Update
          (Transformation|SetRelativeLocation _hammer (Math|Vector|MakeVector (* _bewegung -8e+01) 0.0 (* _bewegung_höhe -8e+01)) false false)
          (Transformation|SetRelativeRotation _hammer (Math|Rotator|MakeRotator 0.0 (* _rotation 1.2e+02) 0.0) false false))
        (:Finished
          (Components|DestroyComponent (Variables|Default|GetCollider))
          ;[0.15 0.15 0.15 0.5] Steinzersprungen
          (Utilities|FlowControl|Sequence
            (:then_0
              (Utilities|FlowControl|Delay 0.3)
              (Components|DestroyComponent (Variables|Default|GetHammer))
              (CallFunction|ReturntoCharacter)
              (bind _asbp_hammer (Utilities|Casting|CastToBP_Hammer (Variables|/Game/BluePrints/Character/BP_PlayerCharacter.BP_PlayerCharacter_C|GetObyect%20in%20Hand (Variables|Default|GetPlayer%20CHaracter))))
              (Default|SetVisibility _asbp_hammer))
            (:then_1
              (Physics|SetSimulatePhysics _gc_1_skulptet_block2 true)
              (Physics|AddImpulse _gc_1_skulptet_block2 "0.000000,0.000000,300000.000000" "None" false)
              (Utilities|FlowControl|Delay 1.0)
              (bind _newtrack_0 (Timeline|Scale PlayFromStart)
                (:Update
                  (Transformation|SetWorldScale3D _gc_1_skulptet_block2 (Math|Vector|MakeVector _newtrack_0 _newtrack_0 _newtrack_0)))
                (:Finished
                  (Utilities|IsValid _actor_destroy
                    (:Is%20Valid
                      (Actor|DestroyActor _actor_destroy))
                    (:Is%20Not%20Valid
                      _))
                  (Actor|DestroyActor))))))))))

(fn ConstructionScript)