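; Base Blueprint for hammer puzzle interactables, built on an inherited pickup interaction.
; On InteractPickup it runs the parent logic, then calls SetVisibility on the player's held object if that is a BP_Hammer.
; The IA_PuzzleExit input returns to the character and waits out the smooth process duration, with nothing after the delay.
; A second hammer visibility call is left disconnected and never runs.
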(event Input|EnhancedActionEvents|EnhancedInputActionIA_PuzzleExit
  (params (ActionValue :type Boolean) (ElapsedSeconds :type Float%20%28double-precision%29) (TriggeredSeconds :type Float%20%28double-precision%29) (InputAction :type Input%20Action%20Object%20Reference :default "/Game/Input/Rätzel/IA_PuzzleExit.IA_PuzzleExit"))
  (CallFunction|ReturntoCharacter)
  (Utilities|FlowControl|Delay (Variables|Default|GetSmooth%20Prosess%20Duration)))

(event EventInteractPickup
  (params (PlayerCharacter :type BP%20Player%20Character%20Object%20Reference) (WillPlayerWatchingObjectInHand? :type Boolean) (IsObjectInHand? :type Boolean))
  (|CallParentFunction PlayerCharacter WillPlayerWatchingObjectInHand? IsObjectInHand?)
  (bind _asbp_hammer (Utilities|Casting|CastToBP_Hammer (Variables|/Game/BluePrints/Character/BP_PlayerCharacter.BP_PlayerCharacter_C|GetObyect%20in%20Hand (Variables|Default|GetPlayer%20CHaracter))))
  (Default|SetVisibility _asbp_hammer))

(fn ConstructionScript)