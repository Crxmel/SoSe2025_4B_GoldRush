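; Interactable generator for the hammer puzzle that switches on the level's BP_LichtParent lights.
; Interaction requires the linked BP_Latte1 plank to be broken (LatteKaputt), otherwise it shows a tutorial UI hint.
; The one-time power-up loops over all lights with delays, plays the generator sound, calls GenAn and returns control to the character.
; DebugStromAn triggers the same sequence at BeginPlay, skipping the character return.
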(event EventBeginPlay
  (|CallParentFunction)
  (if (Variables|Default|GetDebug_StromAn)
    (Utilities|FlowControl|Delay (Variables|Default|GetLichtAnDelay))
    (bind _outactors (Actor|GetAllActorsOfClass "/Game/BluePrints/Licht/BP_LichtParent.BP_LichtParent_C"))
    (for _array_element _outactors
      (bind _asbp_licht_parent (Utilities|Casting|CastToBP_LichtParent _array_element))
      (Default|Lichton _asbp_licht_parent)
      (Utilities|FlowControl|Delay (Variables|Default|GetLichtAnDelay))
      (Audio|Components|Audio|Play (Variables|Default|GetSC_Generator) 0.0)
      (Default|CallGenAn)
      (if (not (Variables|Default|GetDebug_StromAn))
        (CallFunction|ReturntoCharacter)))))

(event EventGetProsses
  (params (Player%20CHaracter :type BP%20Player%20Character%20Object%20Reference) (In%20Pawn :type Pawn%20Object%20Reference))
  (bind _asbp_latte_1 (Utilities|Casting|CastToBP_Latte1 (Variables|Default|GetBP_Latte)))
  (if (Variables|/Game/BluePrints/Interactable/HammerRätzel/BP_Latte1.BP_Latte1_C|GetLatteKaputt _asbp_latte_1)
    (Utilities|FlowControl|DoOnce false
      (:Completed
        (|CallParentFunction 0 0)
        (Utilities|FlowControl|Delay (Variables|Default|GetLichtAnDelay))
        (bind _outactors (Actor|GetAllActorsOfClass "/Game/BluePrints/Licht/BP_LichtParent.BP_LichtParent_C"))
        (for _array_element _outactors
          (bind _asbp_licht_parent (Utilities|Casting|CastToBP_LichtParent _array_element))
          (Default|Lichton _asbp_licht_parent)
          (Utilities|FlowControl|Delay (Variables|Default|GetLichtAnDelay))
          (Audio|Components|Audio|Play (Variables|Default|GetSC_Generator) 0.0)
          (Default|CallGenAn)
          (if (not (Variables|Default|GetDebug_StromAn))
            (CallFunction|ReturntoCharacter)))))
    (else
      (Default|GenTotorial (Variables|/Game/BluePrints/Character/BP_PlayerCharacter.BP_PlayerCharacter_C|GetMainUI (Variables|Default|GetPlayer%20CHaracter))))))

(fn ConstructionScript
  (|CallParentFunction))