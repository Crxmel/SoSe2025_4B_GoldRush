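; BP_Hammer is a hammer pickup in the HammerRätzel interactable set.
; It extends the parent InteractPickup, printing German debug messages for pickup and drop and keeping the capsule at query and physics collision in both cases.
; Pickup sets PlayerHasHammer on the player character, and dropping leaves that flag untouched.
; SetVisibility applies the Visebliti flag to the cube and hammer components, then flips it for the next call.
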(event Custom|SetVisibility
  (Rendering|SetVisibility (Variables|Default|GetCube) (Variables|Default|GetVisebliti) false)
  (Variables|Default|SetVisebliti (not (Variables|Default|GetVisebliti))))

(event EventInteractPickup
  (params (PlayerCharacter :type BP%20Player%20Character%20Object%20Reference) (WillPlayerWatchingObjectInHand? :type Boolean) (IsObjectInHand? :type Boolean) (IsPosessesBlockt? :type Boolean))
  (|CallParentFunction PlayerCharacter WillPlayerWatchingObjectInHand? IsObjectInHand? false)
  (if IsObjectInHand?
    (Development|PrintString "Hammer fallen gelassen")
    (Collision|SetCollisionEnabled (Variables|Default|GetCapsule) "QueryAndPhysics")
    (else
      (Development|PrintString "Hammer aufgehoben")
      (Variables|/Game/BluePrints/Character/BP_PlayerCharacter.BP_PlayerCharacter_C|SetPlayerHasHammer? (Variables|Default|GetPlayer%20Character) true)
      (Collision|SetCollisionEnabled (Variables|Default|GetCapsule) "QueryAndPhysics"))))

(fn ConstructionScript)