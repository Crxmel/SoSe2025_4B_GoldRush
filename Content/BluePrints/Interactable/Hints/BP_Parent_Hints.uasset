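; Base Blueprint for pickup hint objects that display up to twelve lines of text in the game.
; The construction script copies the text variables into their matching line components.
; Picking it up runs the parent interaction and turns on button prompts in the player's main UI.
; BeginPlay stores the starting location, and ChildReset detaches the hint, returns it there and zeroes its relative rotation.
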(event EventBeginPlay
  (Variables|Default|SetLocaitionTo%20snap (Transformation|GetWorldLocation (Variables|Default|GetScene))))

(event Collision|EventActorBeginOverlap
  (params (OtherActor :type Actor%20Object%20Reference)))

(event EventTick
  (params (DeltaSeconds :type Float%20%28single-precision%29)))

(event EventInteractPickup
  (params (PlayerCharacter :type BP%20Player%20Character%20Object%20Reference) (WillPlayerWatchingObjectInHand? :type Boolean) (IsObjectInHand? :type Boolean) (IsPosessesBlockt? :type Boolean))
  (|CallParentFunction PlayerCharacter WillPlayerWatchingObjectInHand? IsObjectInHand? IsPosessesBlockt?)
  (Default|TotoButton (Variables|/Game/BluePrints/Character/BP_PlayerCharacter.BP_PlayerCharacter_C|GetMainUI PlayerCharacter) true false true false true false true))

(event EventChildReset
  (Transformation|DetachFromActor "KeepWorld" "KeepWorld" "KeepWorld")
  (Transformation|SetActorLocation (Variables|Default|GetLocaitionTo%20snap) false false)
  (Transformation|SetActorRelativeRotation "0, 0, 0")
  (if (Variables|Default|GetFinige%20Game)
    _))

(fn ConstructionScript
  (|CallParentFunction)
  (Rendering|Components|TextRender|SetText (Variables|Default|GetZeile%201) (Variables|Text|GetZeile_1))
  (Rendering|Components|TextRender|SetText (Variables|Default|GetZeile%202) (Variables|Text|GetZeile_2))
  (Rendering|Components|TextRender|SetText (Variables|Default|GetZeile%203) (Variables|Text|GetZeile_3))
  (Rendering|Components|TextRender|SetText (Variables|Default|GetZeile%204) (Variables|Text|GetZeile_4))
  (Rendering|Components|TextRender|SetText (Variables|Default|GetZeile%205) (Variables|Text|GetZeile_5))
  (Rendering|Components|TextRender|SetText (Variables|Default|GetZeile%206) (Variables|Text|GetZeile_6))
  (Rendering|Components|TextRender|SetText (Variables|Default|GetZeile%207) (Variables|Text|GetZeile_7))
  (Rendering|Components|TextRender|SetText (Variables|Default|GetZeile%208) (Variables|Text|GetZeile_8))
  (Rendering|Components|TextRender|SetText (Variables|Default|GetZeile%209) (Variables|Text|GetZeile_9))
  (Rendering|Components|TextRender|SetText (Variables|Default|GetZeile%2010) (Variables|Text|GetZeile_10))
  (Rendering|Components|TextRender|SetText (Variables|Default|GetZeile%2011) (Variables|Text|GetZeile_11))
  (Rendering|Components|TextRender|SetText (Variables|Default|GetZeile%2012) (Variables|Text|GetZeile_12)))