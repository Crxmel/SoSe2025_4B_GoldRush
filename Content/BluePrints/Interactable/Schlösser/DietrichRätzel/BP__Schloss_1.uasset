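; Interactable lockpick puzzle: a player holding a lockpick (Dietrich) rotates the lock (Schloss) to find a target angle.
; Interaction calls the parent pickup logic and shows the pick; mouse input rolls the lock, and exit returns to the character.
; Tick drives a DoOnce-gated Timeline that rotates the pick when roll is within the tolerance around the solution.
; The action input checks that range; success exits, then after a delay destroys the actor and clears the player's lockpick flag.
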(event Custom|DietrichPuzzleFinish
  (CallFunction|ReturntoCharacter)
  (Rendering|SetVisibility (Variables|Default|GetDietrich) false false))

(event Input|EnhancedActionEvents|EnhancedInputActionIA_PuzzleExit
  (params (ActionValue :type Boolean) (ElapsedSeconds :type Float%20%28double-precision%29) (TriggeredSeconds :type Float%20%28double-precision%29) (InputAction :type Input%20Action%20Object%20Reference :default "/Game/Input/Rätzel/IA_PuzzleExit.IA_PuzzleExit"))
  (CallFunction|ReturntoCharacter)
  (Rendering|SetVisibility (Variables|Default|GetDietrich) false false))

(event Input|EnhancedActionEvents|EnhancedInputActionIA_PuzzleMous
  (params (ActionValue :type Vector%202D%20Structure) (ElapsedSeconds :type Float%20%28double-precision%29) (TriggeredSeconds :type Float%20%28double-precision%29) (InputAction :type Input%20Action%20Object%20Reference :default "/Game/Input/Rätzel/IA_PuzzleMous.IA_PuzzleMous"))
  (Transformation|AddRelativeRotation (Variables|Default|GetSchloss) (Math|Rotator|MakeRotator (.x ActionValue) 0.0 0.0) false false))

(event Input|EnhancedActionEvents|EnhancedInputActionIA_PuzzleAction
  (params (ActionValue :type Boolean) (ElapsedSeconds :type Float%20%28double-precision%29) (TriggeredSeconds :type Float%20%28double-precision%29) (InputAction :type Input%20Action%20Object%20Reference :default "/Game/Input/Rätzel/IA_PuzzleAction.IA_PuzzleAction"))
  (bind _schloss (Variables|Default|GetSchloss))
  (bind _returnvalue (Transformation|GetWorldRotation _schloss))
  (if (and (> (.roll _returnvalue) (- (Variables|Default|GetLösungswert) (/ (Variables|Default|GetSpannweite) 2))) (< (.roll _returnvalue) (+ (Variables|Default|GetLösungswert) (/ (Variables|Default|GetSpannweite) 2))))
    (Development|PrintString "Richtig" true true "(R=0.000000,G=1.000000,B=0.116116,A=1.000000)")
    (CallFunction|DietrichPuzzleFinish)
    (Utilities|FlowControl|Delay (Variables|Default|GetSmooth%20Prosess%20Duration))
    (Actor|DestroyActor)
    (Variables|/Game/BluePrints/Character/BP_PlayerCharacter.BP_PlayerCharacter_C|SetPlayerHasDietrich (Variables|Default|GetPlayer%20CHaracter) false)
    (else
      (Development|PrintString "Falsch" true true "(R=1.000000,G=0.000000,B=0.122453,A=1.000000)"))))

(event EventInteractPickup
  (params (PlayerCharacter :type BP%20Player%20Character%20Object%20Reference) (WillPlayerWatchingObjectInHand? :type Boolean) (IsObjectInHand? :type Boolean))
  (if (Variables|/Game/BluePrints/Character/BP_PlayerCharacter.BP_PlayerCharacter_C|GetPlayerHasDietrich PlayerCharacter)
    (|CallParentFunction PlayerCharacter false false)
    (Rendering|SetVisibility (Variables|Default|GetDietrich) true false)
    (else
      (Development|PrintString "Player Dont Has Dietrich" true true "(R=1.000000,G=0.018618,B=0.000000,A=1.000000)" 5.0))))

(event EventTick
  (params (DeltaSeconds :type Float%20%28single-precision%29))
  (bind _schloss (Variables|Default|GetSchloss))
  (bind _returnvalue (Transformation|GetWorldRotation _schloss))
  ;[0.15 0.15 0.15 0.5] ditrichAnimation
  (if (and (> (.roll _returnvalue) (- (Variables|Default|GetLösungswert) (/ (Variables|Default|GetSpannweite) 2))) (< (.roll _returnvalue) (+ (Variables|Default|GetLösungswert) (/ (Variables|Default|GetSpannweite) 2))))
    (Development|PrintString "Play animation" true true "(R=0.006852,G=0.285417,B=0.000000,A=1.000000)" 0.0)
    (Utilities|FlowControl|DoOnce false :!label _label
      (:Completed
        (Utilities|FlowControl|Sequence
          (:then_0
            (bind _newtrack_0 (Timeline|Timeline Play)
              (:Update
                (Transformation|AddRelativeRotation (Variables|Default|GetRotationPoint_Dietrich) (Math|Rotator|MakeRotator _newtrack_0 0.0 0.0) false false))))
          (:then_1
            (goto _label_2 Reset)))))
    (else
      (Utilities|FlowControl|DoOnce false :!label _label_2
        (:Completed
          (Utilities|FlowControl|Sequence
            (:then_0
              (goto _label Reset))
            (:then_1
              (Timeline|Timeline Stop))))))))

(fn ConstructionScript
  (|CallParentFunction))