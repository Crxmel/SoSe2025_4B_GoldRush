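; Lockpicking puzzle interactable (Schloss = lock) that shows a lockpick (Dietrich) on interaction and hides it when the player exits back to the character.
; Puzzle mouse input rolls the Scene component, and Tick watches for its world roll entering a fixed angle window.
; The first hit plays a timeline once, adding further roll on each update.
; The action input is a stub with a debug print and an empty angle check.
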(event Input|EnhancedActionEvents|EnhancedInputActionIA_PuzzleExit
  (params (ActionValue :type Boolean) (ElapsedSeconds :type Float%20%28double-precision%29) (TriggeredSeconds :type Float%20%28double-precision%29) (InputAction :type Input%20Action%20Object%20Reference :default "/Game/Input/Rätzel/IA_PuzzleExit.IA_PuzzleExit"))
  (CallFunction|ReturntoCharacter)
  (Rendering|SetVisibility (Variables|Default|GetDietrich) false false))

(event Input|EnhancedActionEvents|EnhancedInputActionIA_PuzzleMous
  (params (ActionValue :type Vector%202D%20Structure) (ElapsedSeconds :type Float%20%28double-precision%29) (TriggeredSeconds :type Float%20%28double-precision%29) (InputAction :type Input%20Action%20Object%20Reference :default "/Game/Input/Rätzel/IA_PuzzleMous.IA_PuzzleMous"))
  (Transformation|AddWorldRotation (Variables|Default|GetScene) (Math|Rotator|MakeRotator (.x ActionValue) 0.0 0.0) false false))

(event Input|EnhancedActionEvents|EnhancedInputActionIA_PuzzleAction
  (params (ActionValue :type Boolean) (ElapsedSeconds :type Float%20%28double-precision%29) (TriggeredSeconds :type Float%20%28double-precision%29) (InputAction :type Input%20Action%20Object%20Reference :default "/Game/Input/Rätzel/IA_PuzzleAction.IA_PuzzleAction"))
  (bind _scene (Variables|Default|GetScene))
  (bind _returnvalue (Transformation|GetWorldRotation _scene))
  (Development|PrintString "Hello")
  (if (and (> (.roll _returnvalue) 1e+02) (< (.roll _returnvalue) 1.2e+02))
    _))

(event EventInteractPickup
  (params (PlayerCharacter :type BP%20Player%20Character%20Object%20Reference) (WillPlayerWatchingObjectInHand? :type Boolean) (IsObjectInHand? :type Boolean))
  (|CallParentFunction PlayerCharacter false false)
  (Rendering|SetVisibility (Variables|Default|GetDietrich) true false))

(event EventTick
  (params (DeltaSeconds :type Float%20%28single-precision%29))
  (bind _scene (Variables|Default|GetScene))
  (bind _returnvalue (Transformation|GetWorldRotation _scene))
  (if (and (> (.roll _returnvalue) 1e+02) (< (.roll _returnvalue) 1.2e+02))
    (Utilities|FlowControl|DoOnce false
      (:Completed
        (Development|PrintString "Play")
        (bind _newtrack_0 (Timeline|Timeline Play)
          (:Update
            (Transformation|AddWorldRotation (Variables|Default|GetScene) (Math|Rotator|MakeRotator (+ 0.0 _newtrack_0) 0.0 0.0) false false)))))))

(fn ConstructionScript
  (|CallParentFunction))