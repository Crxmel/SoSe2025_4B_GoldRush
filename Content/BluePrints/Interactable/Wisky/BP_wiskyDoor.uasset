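; Door for the whisky puzzle that destroys itself to open after three OpenDoor signals.
; On BeginPlay it binds one event to the OpenDoor dispatcher of three puzzle placement actors.
; Chained DoOnce gates act as a counter, each unlocking the next after a short delay, so signals arriving during that delay do not advance it.
; It counts signals without checking which placement sent them.
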(event Custom|Open%20Door_Event
  (Utilities|FlowControl|Sequence
    (:then_0
      (Utilities|FlowControl|DoOnce false
        (:Completed
          (Utilities|FlowControl|Delay 0.2)
          (goto _label Reset))))
    (:then_1
      (Utilities|FlowControl|DoOnce true :!label _label
        (:Completed
          (Utilities|FlowControl|Delay 0.2)
          (goto _label_2 Reset))))
    (:then_2
      (Utilities|FlowControl|DoOnce true :!label _label_2
        (:Completed
          (Actor|DestroyActor))))))

(event EventBeginPlay
  (EventDispatchers|AssignOpenDoor (Variables|Default|GetWieskyRätzelPlatzirung_3) (delegate Custom|Open%20Door_Event)))

(fn ConstructionScript)