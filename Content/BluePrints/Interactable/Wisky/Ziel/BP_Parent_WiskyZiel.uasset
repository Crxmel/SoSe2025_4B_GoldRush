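; Parent Blueprint for a whiskey puzzle target that accepts a carried whiskey pickup when its tags match the required tag.
; On interaction it clears the player's held-item flags, snaps the object to a set point and calls OpenDoor.
; A timeline then moves an animation point along Z.
; When the timeline finishes, it plays the animation on the assigned asset, trying casts to three door-puzzle animation Blueprints in turn.
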(event EventInteractPickup
  (params (PlayerCharacter :type BP%20Player%20Character%20Object%20Reference) (WillPlayerWatchingObjectInHand? :type Boolean) (IsObjectInHand? :type Boolean) (IsPosessesBlockt? :type Boolean))
  (bind _assettoanimate (Variables|Default|GetAssetToAnimate))
  (bind _asbp_pickup_parent_wiski (Utilities|Casting|CastToBP_Pickup_ParentWiski (Variables|/Game/BluePrints/Character/BP_PlayerCharacter.BP_PlayerCharacter_C|GetObyect%20in%20Hand PlayerCharacter)))
  (Utilities|IsValid (Actor|GetComponentbyClass _asbp_pickup_parent_wiski "/Game/BluePrints/Interactable/BP_Tags.BP_Tags_C")
    (:Is%20Valid
      (if (GameplayTags|HasTag (Variables|/Game/BluePrints/Interactable/BP_Tags.BP_Tags_C|GetTagContain (Actor|GetComponentbyClass _asbp_pickup_parent_wiski "/Game/BluePrints/Interactable/BP_Tags.BP_Tags_C")) (Variables|Default|GetTagToNeed))
        (Variables|/Game/BluePrints/Character/BP_PlayerCharacter.BP_PlayerCharacter_C|SetPlayerHasWisky? PlayerCharacter false)
        (Variables|/Game/BluePrints/Character/BP_PlayerCharacter.BP_PlayerCharacter_C|SetIsObyectInHand? PlayerCharacter false)
        (Transformation|AttachComponentToComponent (Variables|/Game/BluePrints/Character/BP_PlayerCharacter.BP_PlayerCharacter_C|GetObyect%20in%20Hand PlayerCharacter) (Variables|Default|GetObjectSetPoint) "None" "SnapToTarget" "SnapToTarget" "KeepWorld" true)
        (Default|CallOpenDoor)
        (bind _newtrack_0 (Timeline|Timeline PlayFromStart)
          (:Update
            (Transformation|SetRelativeLocation (Variables|Default|GetAnimationspoint) (Math|Vector|MakeVector 0.0 0.0 (* _newtrack_0 -3.0)) false false))
          (:Finished
            ;[0.15 0.15 0.15 0.5] AnimationTrigger
            (bind _asbp_animation_doorretzel_draußen (Utilities|Casting|CastToBP_Animation_Doorretzel_Draußen _assettoanimate)
              (:then
                (Default|AnimationPlay _asbp_animation_doorretzel_draußen))
              (:CastFailed
                (bind _asbp_animation_doorretzel_teke (Utilities|Casting|CastToBP_Animation_Doorretzel_Teke _assettoanimate)
                  (:then
                    (Default|AnimationPlay _asbp_animation_doorretzel_teke))
                  (:CastFailed
                    (bind _asbp_animation_doorretzel_tisch (Utilities|Casting|CastToBP_Animation_Doorretzel_Tisch _assettoanimate))
                    (Default|AnimationPlay _asbp_animation_doorretzel_tisch)))))))))))

(fn ConstructionScript
  (|CallParentFunction))