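; Whisky glass pickup Blueprint that sets which of its glass components is visible when play begins.
; After the parent BeginPlay, it hides Glas03, then shows Glas01 if its BPTags tag container has the Wisky_02 tag, or Glas02 otherwise.
; The construction script only calls the parent, and no pickup logic is defined in these graphs.
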(event EventBeginPlay
  (|CallParentFunction)
  (Rendering|SetVisibility (Variables|Default|GetGlas_03) false false)
  (if (GameplayTags|HasTag (Variables|/Game/BluePrints/Interactable/BP_Tags.BP_Tags_C|GetTagContain (Variables|Default|GetBP_Tags)) "(TagName=\"Wisky_02\")")
    (Rendering|SetVisibility (Variables|Default|GetGlas_01) true false)
    (else
      (Rendering|SetVisibility (Variables|Default|GetGlas_02) true false))))

(fn ConstructionScript
  (|CallParentFunction))