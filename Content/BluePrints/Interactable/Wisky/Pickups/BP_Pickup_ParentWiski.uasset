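; Base Blueprint for whisky pickups, extending a parent pickup's interaction to flag the player as holding whisky.
; On BeginPlay it registers a gameplay tag and caches its Scene component's world location as a snap point.
; Interaction runs the parent pickup logic and sets the player flag only when IsObjectInHand is false.
; Childreset detaches the pickup, returns it to the cached location and zeroes its relative rotation.
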(event Custom|Child%20reset
  (Transformation|DetachFromActor "KeepWorld" "KeepWorld" "KeepWorld")
  (Transformation|SetActorLocation (Variables|Default|GetLocaitionTo%20snap) false false)
  (Transformation|SetActorRelativeRotation "0, 0, 0"))

(event EventBeginPlay
  (GameplayTags|AddGameplayTag (Variables|/Game/BluePrints/Interactable/BP_Tags.BP_Tags_C|GetTagContain (Variables|Default|GetBP_Tags)) (Variables|Default|GetTag) :!class /Script/GameplayTags.BlueprintGameplayTagLibrary)
  (Variables|Default|SetLocaitionTo%20snap (Transformation|GetWorldLocation (Variables|Default|GetScene))))

(event EventInteractPickup
  (params (PlayerCharacter :type BP%20Player%20Character%20Object%20Reference) (WillPlayerWatchingObjectInHand? :type Boolean) (IsObjectInHand? :type Boolean) (IsPosessesBlockt? :type Boolean))
  (if (not IsObjectInHand?)
    (|CallParentFunction PlayerCharacter WillPlayerWatchingObjectInHand? IsObjectInHand? false)
    (Variables|/Game/BluePrints/Character/BP_PlayerCharacter.BP_PlayerCharacter_C|SetPlayerHasWisky? (Variables|Default|GetPlayer%20Character) true)))

(fn ConstructionScript
  (|CallParentFunction))