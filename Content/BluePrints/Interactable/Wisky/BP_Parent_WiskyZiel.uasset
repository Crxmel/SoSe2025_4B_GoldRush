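; BP_Parent_WiskyZiel is a parent Blueprint for an interactable target where the player deposits a carried whisky pickup.
; On InteractPickup it casts the held object to BP_Pickup_ParentWiski and checks that its BP_Tags component's container matches TagToNeed, non-exactly.
; On a match it clears the player's whisky and in-hand flags, then snaps the object to ObjectSetPoint, keeping world scale.
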(event EventInteractPickup
  (params (PlayerCharacter :type BP%20Player%20Character%20Object%20Reference) (WillPlayerWatchingObjectInHand? :type Boolean) (IsObjectInHand? :type Boolean))
  (bind _asbp_pickup_parent_wiski (Utilities|Casting|CastToBP_Pickup_ParentWiski (Variables|/Game/BluePrints/Character/BP_PlayerCharacter.BP_PlayerCharacter_C|GetObyect%20in%20Hand PlayerCharacter)))
  (Utilities|IsValid (Actor|GetComponentbyClass _asbp_pickup_parent_wiski "/Game/BluePrints/Interactable/Wisky/BP_Tags.BP_Tags_C")
    (:Is%20Valid
      (if (GameplayTags|HasTag (Variables|/Game/BluePrints/Interactable/Wisky/BP_Tags.BP_Tags_C|GetTagContain (Actor|GetComponentbyClass _asbp_pickup_parent_wiski "/Game/BluePrints/Interactable/Wisky/BP_Tags.BP_Tags_C")) (Variables|Default|GetTagToNeed))
        (Variables|/Game/BluePrints/Character/BP_PlayerCharacter.BP_PlayerCharacter_C|SetPlayerHasWisky? PlayerCharacter false)
        (Variables|/Game/BluePrints/Character/BP_PlayerCharacter.BP_PlayerCharacter_C|SetIsObyectInHand? PlayerCharacter false)
        (Transformation|AttachComponentToComponent (Variables|/Game/BluePrints/Character/BP_PlayerCharacter.BP_PlayerCharacter_C|GetObyect%20in%20Hand PlayerCharacter) (Variables|Default|GetObjectSetPoint) "None" "SnapToTarget" "SnapToTarget" "KeepWorld" true)))))

(fn ConstructionScript
  (|CallParentFunction))