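; BP_Drehdings_02 is an interactable rotary combination-lock puzzle with four dial components held in an array.
; Puzzle-navigate up and down inputs set a direction and play a shared timeline that rolls the selected dial one 36-degree step.
; InputBlock, which allows input when true, gates presses until the timeline finishes and saves the roll.
; This graph contains no selection switching or solution check.
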(event Input|EnhancedActionEvents|EnhancedInputActionIA_PuzzleNavigate_Up
  (params (ActionValue :type Boolean) (ElapsedSeconds :type Float%20%28double-precision%29) (TriggeredSeconds :type Float%20%28double-precision%29) (InputAction :type Input%20Action%20Object%20Reference :default "/Game/Input/Rätzel/IA_PuzzleNavigate_Up.IA_PuzzleNavigate_Up"))
  (if (Variables|Default|GetInputBlock)
    (Variables|Default|SetInputBlock (not (Variables|Default|GetInputBlock)))
    (Variables|Default|SetRotationUp/Down 1.0)
    (bind _newtrack_0 (Timeline|Timeline PlayFromStart)
      (:Update
        (Transformation|SetRelativeRotation (CallFunction|GetSelectedButton) (Math|Rotator|MakeRotator (+ (* (* _newtrack_0 (Variables|Default|GetRotationUp/Down)) 36.0) (Variables|Default|GetRotationSave)) 0.0 0.0) false false))
      (:Finished
        (Variables|Default|SetRotationSave (.roll (Variables|/Script/Engine.SceneComponent|GetRelativeRotation (CallFunction|GetSelectedButton))))
        (Variables|Default|SetInputBlock true)))))

(event Input|EnhancedActionEvents|EnhancedInputActionIA_PuzzleNavigate_Down
  (params (ActionValue :type Boolean) (ElapsedSeconds :type Float%20%28double-precision%29) (TriggeredSeconds :type Float%20%28double-precision%29) (InputAction :type Input%20Action%20Object%20Reference :default "/Game/Input/Rätzel/IA_PuzzleNavigate_Down.IA_PuzzleNavigate_Down"))
  (if (Variables|Default|GetInputBlock)
    (Variables|Default|SetInputBlock (not (Variables|Default|GetInputBlock)))
    (Variables|Default|SetRotationUp/Down -1.0)
    (bind _newtrack_0 (Timeline|Timeline PlayFromStart)
      (:Update
        (Transformation|SetRelativeRotation (CallFunction|GetSelectedButton) (Math|Rotator|MakeRotator (+ (* (* _newtrack_0 (Variables|Default|GetRotationUp/Down)) 36.0) (Variables|Default|GetRotationSave)) 0.0 0.0) false false))
      (:Finished
        (Variables|Default|SetRotationSave (.roll (Variables|/Script/Engine.SceneComponent|GetRelativeRotation (CallFunction|GetSelectedButton))))
        (Variables|Default|SetInputBlock true)))))

(event EventBeginPlay
  (Variables|Default|SetArray (Utilities|Array|MakeArray (Variables|Default|GetBP_dreh) (Variables|Default|GetBP_dreh1) (Variables|Default|GetBP_dreh2) (Variables|Default|GetBP_dreh3))))

(fn ConstructionScript
  (|CallParentFunction))

(fn GetSelectedButton
  (return (Utilities|Array|Get(acopy) (Variables|Default|GetArray) (Variables|Default|GetSelectedButtonCount))))