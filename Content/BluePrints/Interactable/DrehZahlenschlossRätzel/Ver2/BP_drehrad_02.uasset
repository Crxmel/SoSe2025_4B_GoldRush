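; Rotating number wheel for a combination lock puzzle, stepped one face up or down per Rotate call.
; Rotate updates the selected face index and derives a target pitch from the face count, which Tick smoothly follows via shortest-path rotator lerp.
; ClampSelectedFace wraps the index, though downward wrap lands on NumFaces rather than the last index.
; GetCurrentNumber maps the index to a digit enum.
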(event Custom|Rotate
  (params (Up :type Boolean))
  (bind _output_get (Variables|Default|SetCurrectSelectedFaces (CallFunction|ClampSelectedFace (+ (Variables|Default|GetCurrectSelectedFaces) (Math|Integer|SelectInt 1 -1 Up)))))
  (Variables|Default|SetTargetRot (* (Math|Conversions|ToFloat(Integer) _output_get) (/ 3.6e+02 (Math|Conversions|ToFloat(Integer) (Variables|Default|GetNumFaces))) -1.0)))

(event EventTick
  (params (DeltaSeconds :type Float%20%28single-precision%29))
  (Transformation|SetRelativeRotation (Math|Rotator|Lerp(Rotator) (Variables|Default|GetRelativeRotation) (Math|Rotator|MakeRotator 0.0 (Variables|Default|GetTargetRot) 0.0) (* (Utilities|Time|GetWorldDeltaSeconds) 1e+01) true) false false))

(fn ClampSelectedFace
  (params (input :type Integer))
  (LocalVariables|SetClampIndex input)
  (Utilities|FlowControl|Sequence
    (:then_0
      (if (> (LocalVariables|GetClampIndex) (- (Variables|Default|GetNumFaces) 1))
        (LocalVariables|SetClampIndex 0)))
    (:then_1
      (if (< (LocalVariables|GetClampIndex) 0)
        (LocalVariables|SetClampIndex (- (Variables|Default|GetNumFaces) 0))))
    (:then_2
      (return (LocalVariables|GetClampIndex)))))

(fn GetCurrentNumber
  (return (Utilities|Select :Index (Variables|Default|GetCurrectSelectedFaces) :Option%200 "NewEnumerator1" :Option%201 "NewEnumerator2" :Option%202 "NewEnumerator3" :Option%203 "NewEnumerator4" :Option%204 "NewEnumerator5" :Option%205 "NewEnumerator6" :Option%206 "NewEnumerator7" :Option%207 "NewEnumerator8" :Option%208 "NewEnumerator9" :Option%209 "NewEnumerator0" :Option%2010 "NewEnumerator0")))