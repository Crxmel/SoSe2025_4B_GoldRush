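; BP_Drehschloss is an interactable rotary combination lock puzzle with four dials.
; Puzzle navigation inputs move a clamped selection between dials and rotate the selected one up or down.
; Interact compares each dial to CorrectCode; on a match it returns to the character, waits out the transition, then calls OpenDoor and updates the main UI.
; OpenDoor and the selection-highlight function are empty stubs here.
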(event Custom|OpenDoor)

(event Input|EnhancedActionEvents|EnhancedInputActionIA_PuzzleNavigate_Up
  (params (ActionValue :type Boolean) (ElapsedSeconds :type Float%20%28double-precision%29) (TriggeredSeconds :type Float%20%28double-precision%29) (InputAction :type Input%20Action%20Object%20Reference :default "/Game/Input/Rätzel/IA_PuzzleNavigate_Up.IA_PuzzleNavigate_Up"))
  (Default|Rotate (CallFunction|GetSelectetDisk) true))

(event Input|EnhancedActionEvents|EnhancedInputActionIA_PuzzleNavigate_Down
  (params (ActionValue :type Boolean) (ElapsedSeconds :type Float%20%28double-precision%29) (TriggeredSeconds :type Float%20%28double-precision%29) (InputAction :type Input%20Action%20Object%20Reference :default "/Game/Input/Rätzel/IA_PuzzleNavigate_Down.IA_PuzzleNavigate_Down"))
  (Default|Rotate (CallFunction|GetSelectetDisk) false))

(event Input|EnhancedActionEvents|EnhancedInputActionIA_PuzzleNavigate_Left
  (params (ActionValue :type Boolean) (ElapsedSeconds :type Float%20%28double-precision%29) (TriggeredSeconds :type Float%20%28double-precision%29) (InputAction :type Input%20Action%20Object%20Reference :default "/Game/Input/Rätzel/IA_PuzzleNavigate_Left.IA_PuzzleNavigate_Left"))
  (CallFunction|ChangeSelectedDisk false))

(event Input|EnhancedActionEvents|EnhancedInputActionIA_PuzzleNavigate_Right
  (params (ActionValue :type Boolean) (ElapsedSeconds :type Float%20%28double-precision%29) (TriggeredSeconds :type Float%20%28double-precision%29) (InputAction :type Input%20Action%20Object%20Reference :default "/Game/Input/Rätzel/IA_PuzzleNavigate_Right.IA_PuzzleNavigate_Right"))
  (CallFunction|ChangeSelectedDisk true))

(event Input|EnhancedActionEvents|EnhancedInputActionIA_PuzzleExit
  (params (ActionValue :type Boolean) (ElapsedSeconds :type Float%20%28double-precision%29) (TriggeredSeconds :type Float%20%28double-precision%29) (InputAction :type Input%20Action%20Object%20Reference :default "/Game/Input/Rätzel/IA_PuzzleExit.IA_PuzzleExit"))
  (CallFunction|ReturntoCharacter)
  (Default|TotoButton (Variables|/Game/BluePrints/Character/BP_PlayerCharacter.BP_PlayerCharacter_C|GetMainUI (Variables|Default|GetPlayer%20CHaracter)) false false false false false false false))

(event Input|EnhancedActionEvents|EnhancedInputActionIA_Interact
  (params (ActionValue :type Boolean) (ElapsedSeconds :type Float%20%28double-precision%29) (TriggeredSeconds :type Float%20%28double-precision%29) (InputAction :type Input%20Action%20Object%20Reference :default "/Game/Input/Player/IA_Interact.IA_Interact"))
  (if (CallFunction|CodeCorrect)
    (CallFunction|ReturntoCharacter)
    (Utilities|FlowControl|Delay (Variables|Default|GetSmooth%20Prosess%20Duration))
    (CallFunction|OpenDoor)
    (Default|TotoButton (Variables|/Game/BluePrints/Character/BP_PlayerCharacter.BP_PlayerCharacter_C|GetMainUI (Variables|Default|GetPlayer%20CHaracter)) false false false false false false false)))

(event EventBeginPlay
  (|CallParentFunction)
  (Variables|Default|SetDrehrad (Utilities|Array|MakeArray (Variables|Default|GetBP_drehrad_00) (Variables|Default|GetBP_drehrad_01) (Variables|Default|GetBP_drehrad_02) (Variables|Default|GetBP_drehrad_03))))

(fn ConstructionScript
  (|CallParentFunction))

(fn GetSelectetDisk
  (return (Utilities|Array|Get(acopy) (Variables|Default|GetDrehrad) (Variables|Default|GetSelectedDrehradIndex))))

(fn ChangeSelectedDisk
  (params (Right :type Boolean))
  (Variables|Default|SetSelectedDrehradIndex (Math|Integer|Clamp(Integer) (+ (Variables|Default|GetSelectedDrehradIndex) (Math|Integer|SelectInt 1 -1 Right)) 0 (Utilities|Array|LastIndex (Variables|Default|GetDrehrad)))))

(fn SetSelectedDrehdingsHighlight
  (params (Enable :type Boolean)))

(fn CodeCorrect
  (for (_array_element _array_index) (Variables|Default|GetDrehrad)
    (if (!= (Default|GetCurrentNumber _array_element) (Utilities|Array|Get(acopy) (Variables|Default|GetCorrectCode) _array_index))
      (return false)))
  (return true))