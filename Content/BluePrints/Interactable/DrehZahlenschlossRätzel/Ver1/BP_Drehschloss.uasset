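; BP_Drehschloss is an interactable combination lock puzzle with four rotating dials that opens a door when solved.
; Left/right input cycles the highlighted dial via an overlay material, while up/down turns it one step on a shared Timeline with input blocked during the animation.
; Interact compares each dial's symbol enum against CorrectCode; on a match it returns to the character, calls the door open and destroys itself after a delay.
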(event Input|EnhancedActionEvents|EnhancedInputActionIA_PuzzleExit
  (params (ActionValue :type Boolean) (ElapsedSeconds :type Float%20%28double-precision%29) (TriggeredSeconds :type Float%20%28double-precision%29) (InputAction :type Input%20Action%20Object%20Reference :default "/Game/Input/Rätzel/IA_PuzzleExit.IA_PuzzleExit"))
  (CallFunction|ReturntoCharacter)
  (CallFunction|UpdateActiveButtonforHightLight false))

(event Input|EnhancedActionEvents|EnhancedInputActionIA_PuzzleNavigate_Left
  (params (ActionValue :type Boolean) (ElapsedSeconds :type Float%20%28double-precision%29) (TriggeredSeconds :type Float%20%28double-precision%29) (InputAction :type Input%20Action%20Object%20Reference :default "/Game/Input/Rätzel/IA_PuzzleNavigate_Left.IA_PuzzleNavigate_Left"))
  (if (not (Variables|Default|GetInputBlock))
    (CallFunction|UpdateActiveButtonforHightLight false)
    (Variables|Default|SetCorrectButtonIndex (- (Variables|Default|GetCorrectButtonIndex) 1))
    (Utilities|FlowControl|Sequence
      (:then_0
        (if (< (Variables|Default|GetCorrectButtonIndex) 0)
          (Variables|Default|SetCorrectButtonIndex (Utilities|Array|LastIndex (Variables|Default|GetButtonArray))))
        (Variables|Default|SetZwischenspeicherRotation (.roll (Variables|/Script/Engine.SceneComponent|GetRelativeRotation (CallFunction|GetActiveButton)))))
      (:then_1
        (CallFunction|UpdateActiveButtonforHightLight true)))))

(event Input|EnhancedActionEvents|EnhancedInputActionIA_PuzzleNavigate_Right
  (params (ActionValue :type Boolean) (ElapsedSeconds :type Float%20%28double-precision%29) (TriggeredSeconds :type Float%20%28double-precision%29) (InputAction :type Input%20Action%20Object%20Reference :default "/Game/Input/Rätzel/IA_PuzzleNavigate_Right.IA_PuzzleNavigate_Right"))
  (if (not (Variables|Default|GetInputBlock))
    (CallFunction|UpdateActiveButtonforHightLight false)
    (Variables|Default|SetCorrectButtonIndex (+ (Variables|Default|GetCorrectButtonIndex) 1))
    (Utilities|FlowControl|Sequence
      (:then_0
        (if (> (Variables|Default|GetCorrectButtonIndex) (Utilities|Array|LastIndex (Variables|Default|GetButtonArray)))
          (Variables|Default|SetCorrectButtonIndex 0))
        (Variables|Default|SetZwischenspeicherRotation (.roll (Variables|/Script/Engine.SceneComponent|GetRelativeRotation (CallFunction|GetActiveButton)))))
      (:then_1
        (CallFunction|UpdateActiveButtonforHightLight true)))))

(event Input|EnhancedActionEvents|EnhancedInputActionIA_PuzzleNavigate_Down
  (params (ActionValue :type Boolean) (ElapsedSeconds :type Float%20%28double-precision%29) (TriggeredSeconds :type Float%20%28double-precision%29) (InputAction :type Input%20Action%20Object%20Reference :default "/Game/Input/Rätzel/IA_PuzzleNavigate_Down.IA_PuzzleNavigate_Down"))
  ;[0.15 0.15 0.15 0.5] Rauf/Runter Rotation
  ;;[0.15 0.15 0.15 0.5] Input blockirt
  (if (not (Variables|Default|GetInputBlock))
    ;;[0.15 0.15 0.15 0.5] Input bloch an
    (Variables|Default|SetInputBlock (not (Variables|Default|GetInputBlock)))
    (Variables|Default|SetRauf/RunterTrigger 1.0)
    (bind _drehung (Timeline|Timeline PlayFromStart)
      (:Update
        (Transformation|SetRelativeRotation (CallFunction|GetActiveButton) (Math|Rotator|MakeRotator (+ (* (* _drehung (Variables|Default|GetRauf/RunterTrigger)) 36.0) (Variables|Default|GetZwischenspeicherRotation)) 0.0 0.0) false false))
      (:Finished
        (Variables|Default|SetZwischenspeicherRotation (.roll (Variables|/Script/Engine.SceneComponent|GetRelativeRotation (CallFunction|GetActiveButton))))
        ;;[0.15 0.15 0.15 0.5] InputBlock aus
        (Variables|Default|SetInputBlock false)))))

(event Input|EnhancedActionEvents|EnhancedInputActionIA_PuzzleNavigate_Up
  (params (ActionValue :type Boolean) (ElapsedSeconds :type Float%20%28double-precision%29) (TriggeredSeconds :type Float%20%28double-precision%29) (InputAction :type Input%20Action%20Object%20Reference :default "/Game/Input/Rätzel/IA_PuzzleNavigate_Up.IA_PuzzleNavigate_Up"))
  ;[0.15 0.15 0.15 0.5] Rauf/Runter Rotation
  ;;[0.15 0.15 0.15 0.5] Input blockirt
  (if (not (Variables|Default|GetInputBlock))
    ;;[0.15 0.15 0.15 0.5] Input bloch an
    (Variables|Default|SetInputBlock (not (Variables|Default|GetInputBlock)))
    (Variables|Default|SetRauf/RunterTrigger -1.0)
    (bind _drehung (Timeline|Timeline PlayFromStart)
      (:Update
        (Transformation|SetRelativeRotation (CallFunction|GetActiveButton) (Math|Rotator|MakeRotator (+ (* (* _drehung (Variables|Default|GetRauf/RunterTrigger)) 36.0) (Variables|Default|GetZwischenspeicherRotation)) 0.0 0.0) false false))
      (:Finished
        (Variables|Default|SetZwischenspeicherRotation (.roll (Variables|/Script/Engine.SceneComponent|GetRelativeRotation (CallFunction|GetActiveButton))))
        ;;[0.15 0.15 0.15 0.5] InputBlock aus
        (Variables|Default|SetInputBlock false)))))

(event Input|EnhancedActionEvents|EnhancedInputActionIA_Interact
  (params (ActionValue :type Boolean) (ElapsedSeconds :type Float%20%28double-precision%29) (TriggeredSeconds :type Float%20%28double-precision%29) (InputAction :type Input%20Action%20Object%20Reference :default "/Game/Input/Player/IA_Interact.IA_Interact"))
  (if (CallFunction|IsCorrectCode)
    (CallFunction|ReturntoCharacter)
    (CallFunction|UpdateActiveButtonforHightLight false)
    (Default|CallOpenDoor)
    (Utilities|FlowControl|Delay (Variables|Default|GetSmooth%20Prosess%20Duration))
    (Actor|DestroyActor)))

(event EventTick
  (params (DeltaSeconds :type Float%20%28single-precision%29))
  (if (Variables|Default|Getdebugdings)
    (Development|PrintString (Utilities|String|ToString(Float) (.roll (Variables|/Script/Engine.SceneComponent|GetRelativeRotation (CallFunction|GetActiveButton)))) true true "(R=0.000000,G=0.660000,B=1.000000,A=1.000000)" 0.0)))

(event EventBeginPlay
  ;[0.15 0.15 0.15 0.5] Set Array
  (Variables|Default|SetButtonArray (Utilities|Array|MakeArray (Variables|Default|GetBP_drehdings_0) (Variables|Default|GetBP_drehdings_1) (Variables|Default|GetBP_drehdings_2) (Variables|Default|GetBP_drehdings_3))))

(event EventInteractPickup
  (params (PlayerCharacter :type BP%20Player%20Character%20Object%20Reference) (WillPlayerWatchingObjectInHand? :type Boolean) (IsObjectInHand? :type Boolean) (IsPosessesBlockt? :type Boolean))
  (|CallParentFunction PlayerCharacter WillPlayerWatchingObjectInHand? IsObjectInHand? false)
  (CallFunction|UpdateActiveButtonforHightLight true))

(fn ConstructionScript
  (|CallParentFunction))

(fn GetActiveButton
  (return (Utilities|Array|Get(acopy) (Variables|Default|GetButtonArray) (Variables|Default|GetCorrectButtonIndex))))

(fn UpdateActiveButtonforHightLight
  (params (Selected :type Boolean))
  (Rendering|Material|SetOverlayMaterial (CallFunction|GetActiveButton) (select Selected "/Game/Material/NewFolder/MI_MaterialButtonHighlight.MI_MaterialButtonHighlight" 0) :!class /Script/Engine.MeshComponent))

(fn IsCorrectCode
  ;[0.15 0.15 0.15 0.5] wenn der loob nicht von der anderen returnnode abgebrochen wurde complitet er mir code richtig
  (for (_array_element _array_index) (Variables|Default|GetButtonArray)
    (if (Variables|Default|Getdebugdings)
      (Development|PrintString (Utilities|String|EnumtoString (Default|GetSymbol _array_element))))
    ;[0.15 0.15 0.15 0.5] controllirt ob der code richtig ist indem der den ricchtigen code vom ESymbol (Enum) vergleicht
    (if (not (== (Default|GetSymbol _array_element) (Utilities|Array|Get(acopy) (Variables|Default|GetCorrectCode) _array_index)))
      ;[0.15 0.15 0.15 0.5] sobald es getriggerd wird wird es abgebrochen
      (return false)))
  (return true))