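; Interactable combination lock puzzle with four rotating symbol dials that opens a door when the correct code is set.
; Left/right input cycles the active dial with an overlay highlight, while up/down turns it 36 degrees through a timeline, gated by InputBlock.
; Interact compares each dial's symbol to CorrectCode; a match returns control to the character, calls the door open and destroys the lock after a delay.
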(event Input|EnhancedActionEvents|EnhancedInputActionIA_PuzzleExit
  (params (ActionValue :type Boolean) (ElapsedSeconds :type Float%20%28double-precision%29) (TriggeredSeconds :type Float%20%28double-precision%29) (InputAction :type Input%20Action%20Object%20Reference :default "/Game/Input/Rätzel/IA_PuzzleExit.IA_PuzzleExit"))
  (CallFunction|ReturntoCharacter)
  (CallFunction|UpdateActiveButtonforHightLight false))

(event Input|EnhancedActionEvents|EnhancedInputActionIA_PuzzleNavigate_Left
  (params (ActionValue :type Boolean) (ElapsedSeconds :type Float%20%28double-precision%29) (TriggeredSeconds :type Float%20%28double-precision%29) (InputAction :type Input%20Action%20Object%20Reference :default "/Game/Input/Rätzel/IA_PuzzleNavigate_Left.IA_PuzzleNavigate_Left"))
  (bind _selectedbutton (CallFunction|GetActiveButton))
  (if (Variables|Default|GetInputBlock)
    (CallFunction|UpdateActiveButtonforHightLight false)
    (Variables|Default|SetCorrectButtonIndex (- (Variables|Default|GetCorrectButtonIndex) 1))
    (Utilities|FlowControl|Sequence
      (:then_0
        (if (< (Variables|Default|GetCorrectButtonIndex) 0)
          (Variables|Default|SetCorrectButtonIndex (Utilities|Array|LastIndex (Variables|Default|GetButtonArray))))
        (Variables|Default|SetZwischenspeicherRotation (.pitch (Variables|/Script/Engine.SceneComponent|GetRelativeRotation _selectedbutton)))
        (Variables|Default|Settest (.pitch (Variables|/Script/Engine.SceneComponent|GetRelativeRotation _selectedbutton))))
      (:then_1
        (CallFunction|UpdateActiveButtonforHightLight true)))))

(event Input|EnhancedActionEvents|EnhancedInputActionIA_PuzzleNavigate_Right
  (params (ActionValue :type Boolean) (ElapsedSeconds :type Float%20%28double-precision%29) (TriggeredSeconds :type Float%20%28double-precision%29) (InputAction :type Input%20Action%20Object%20Reference :default "/Game/Input/Rätzel/IA_PuzzleNavigate_Right.IA_PuzzleNavigate_Right"))
  (bind _selectedbutton (CallFunction|GetActiveButton))
  (bind _relativerotation (Variables|/Script/Engine.SceneComponent|GetRelativeRotation _selectedbutton))
  (if (Variables|Default|GetInputBlock)
    (CallFunction|UpdateActiveButtonforHightLight false)
    (Variables|Default|SetCorrectButtonIndex (+ (Variables|Default|GetCorrectButtonIndex) 1))
    (Utilities|FlowControl|Sequence
      (:then_0
        (if (> (Variables|Default|GetCorrectButtonIndex) (Utilities|Array|LastIndex (Variables|Default|GetButtonArray)))
          (Variables|Default|SetCorrectButtonIndex 0))
        (Variables|Default|SetZwischenspeicherRotation (.pitch _relativerotation))
        (Variables|Default|Settest (.pitch _relativerotation)))
      (:then_1
        (CallFunction|UpdateActiveButtonforHightLight true)))))

(event Input|EnhancedActionEvents|EnhancedInputActionIA_PuzzleNavigate_Down
  (params (ActionValue :type Boolean) (ElapsedSeconds :type Float%20%28double-precision%29) (TriggeredSeconds :type Float%20%28double-precision%29) (InputAction :type Input%20Action%20Object%20Reference :default "/Game/Input/Rätzel/IA_PuzzleNavigate_Down.IA_PuzzleNavigate_Down"))
  (if (Variables|Default|GetInputBlock)
    (Variables|Default|SetInputBlock (not (Variables|Default|GetInputBlock)))
    (Variables|Default|SetRauf/RunterTrigger -1.0)
    (bind _newtrack_0 (Timeline|Timeline_0 PlayFromStart)
      (:Update
        (Transformation|SetRelativeRotation (CallFunction|GetActiveButton) (Math|Rotator|MakeRotator 0.0 (+ (* (* _newtrack_0 (Variables|Default|GetRauf/RunterTrigger)) 36.0) (Variables|Default|Gettest)) 0.0) false false))
      (:Finished
        (Variables|Default|Settest (+ (* (Variables|Default|GetRauf/RunterTrigger) 36.0) (Variables|Default|Gettest)))
        (Variables|Default|SetInputBlock true)))))

(event Input|EnhancedActionEvents|EnhancedInputActionIA_PuzzleNavigate_Up
  (params (ActionValue :type Boolean) (ElapsedSeconds :type Float%20%28double-precision%29) (TriggeredSeconds :type Float%20%28double-precision%29) (InputAction :type Input%20Action%20Object%20Reference :default "/Game/Input/Rätzel/IA_PuzzleNavigate_Up.IA_PuzzleNavigate_Up"))
  (if (Variables|Default|GetInputBlock)
    (Variables|Default|SetInputBlock (not (Variables|Default|GetInputBlock)))
    (Variables|Default|SetRauf/RunterTrigger 1.0)
    (bind _newtrack_0 (Timeline|Timeline_0 PlayFromStart)
      (:Update
        (Transformation|SetRelativeRotation (CallFunction|GetActiveButton) (Math|Rotator|MakeRotator 0.0 (+ (* (* _newtrack_0 (Variables|Default|GetRauf/RunterTrigger)) 36.0) (Variables|Default|Gettest)) 0.0) false false))
      (:Finished
        (Variables|Default|Settest (+ (* (Variables|Default|GetRauf/RunterTrigger) 36.0) (Variables|Default|Gettest)))
        (Variables|Default|SetInputBlock true)))))

(event Input|EnhancedActionEvents|EnhancedInputActionIA_Interact
  (params (ActionValue :type Boolean) (ElapsedSeconds :type Float%20%28double-precision%29) (TriggeredSeconds :type Float%20%28double-precision%29) (InputAction :type Input%20Action%20Object%20Reference :default "/Game/Input/Player/IA_Interact.IA_Interact"))
  (if (CallFunction|IsCorrectCode)
    (CallFunction|ReturntoCharacter)
    (CallFunction|UpdateActiveButtonforHightLight false)
    (Default|CallOpenDoor)
    (Utilities|FlowControl|Delay (Variables|Default|GetSmooth%20Prosess%20Duration))
    (Actor|DestroyActor)))

(event EventTick
  (params (DeltaSeconds :type Float%20%28single-precision%29)))

(event EventBeginPlay
  ;[0.15 0.15 0.15 0.5] Set Array
  (Variables|Default|SetButtonArray (Utilities|Array|MakeArray (Variables|Default|GetBP_drehdings_00) (Variables|Default|GetBP_drehdings_01) (Variables|Default|GetBP_drehdings_02) (Variables|Default|GetBP_drehdings_03))))

(event EventInteractPickup
  (params (PlayerCharacter :type BP%20Player%20Character%20Object%20Reference) (WillPlayerWatchingObjectInHand? :type Boolean) (IsObjectInHand? :type Boolean) (IsPosessesBlockt? :type Boolean))
  (|CallParentFunction PlayerCharacter WillPlayerWatchingObjectInHand? IsObjectInHand? false)
  (CallFunction|UpdateActiveButtonforHightLight true))

(fn ConstructionScript
  (|CallParentFunction))

(fn GetActiveButton
  (return (Utilities|Array|Get(acopy) (Variables|Default|GetButtonArray) (Variables|Default|GetCorrectButtonIndex))))

(fn UpdateActiveButtonforHightLight
  (params (Selected :type Boolean))
  (Rendering|Material|SetOverlayMaterial (CallFunction|GetActiveButton) (select Selected "/Game/Material/NewFolder/MI_MaterialButtonHighlight.MI_MaterialButtonHighlight" 0) :!class /Script/Engine.MeshComponent))

(fn IsCorrectCode
  ;[0.15 0.15 0.15 0.5] wenn der loob nicht von der anderen returnnode abgebrochen wurde complitet er mir code richtig
  (for (_array_element _array_index) (Variables|Default|GetButtonArray)
    (if (Variables|Default|Getdebugdings)
      (Development|PrintString (Utilities|String|EnumtoString (Default|GetSymbol _array_element))))
    ;[0.15 0.15 0.15 0.5] controllirt ob der code richtig ist indem der den ricchtigen code vom ESymbol (Enum) vergleicht
    (if (not (== (Default|GetSymbol _array_element) (Utilities|Array|Get(acopy) (Variables|Default|GetCorrectCode) _array_index)))
      ;[0.15 0.15 0.15 0.5] sobald es getriggerd wird wird es abgebrochen
      (return false)))
  (return true))