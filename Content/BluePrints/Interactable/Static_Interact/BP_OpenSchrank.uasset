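; Interactable cabinet (Schrank) whose four doors swing open and closed on alternate InteractPickup events.
; A FlipFlop plays one Timeline forward or in reverse, and its track drives the relative yaw of each door, mirrored left to right, with one pair swinging wider than the other.
; An input-block flag set during timeline updates ignores further interaction until the animation finishes.
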(event EventInteractPickup
  (params (PlayerCharacter :type BP%20Player%20Character%20Object%20Reference) (WillPlayerWatchingObjectInHand? :type Boolean) (IsObjectInHand? :type Boolean) (IsPosessesBlockt? :type Boolean))
  (if (not (Variables|Default|GetInputBlockIsOn))
    (Utilities|FlowControl|FlipFlop
      (:A
        (bind _newtrack_0 (Timeline|Timeline PlayFromStart)
          (:Update
            (Variables|Default|SetInputBlockIsOn true)
            (Transformation|SetRelativeRotation (Variables|Default|GetTür_LL) (Math|Rotator|MakeRotator 0.0 0.0 (* _newtrack_0 1.1e+02)) false false)
            (Transformation|SetRelativeRotation (Variables|Default|GetTür_RR) (Math|Rotator|MakeRotator 0.0 0.0 (* (* _newtrack_0 1.1e+02) -1.0)) false false)
            (Transformation|SetRelativeRotation (Variables|Default|GetTÜr_R) (Math|Rotator|MakeRotator 0.0 0.0 (* (* _newtrack_0 8e+01) 2.0)) false false)
            (Transformation|SetRelativeRotation (Variables|Default|GetTür_L) (Math|Rotator|MakeRotator 0.0 0.0 (* (* (* _newtrack_0 8e+01) 2.0) -1.0)) false false))
          (:Finished
            (Variables|Default|SetInputBlockIsOn false))))
      (:B
        (Timeline|Timeline ReverseFromEnd)))))

(fn ConstructionScript
  (|CallParentFunction))