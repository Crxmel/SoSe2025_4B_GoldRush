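; BP_OpenKiste is an interactable wooden chest whose lid opens once when interacted with.
; The InteractPickup event passes through a DoOnce that is never reset, then starts the SCHolzkiste sound and a timeline.
; The timeline's Rotate track drives the relative pitch of the KistenDeggel lid, scaled by -100 degrees, and stops the sound when finished.
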(event EventInteractPickup
  (params (PlayerCharacter :type BP%20Player%20Character%20Object%20Reference) (WillPlayerWatchingObjectInHand? :type Boolean) (IsObjectInHand? :type Boolean) (IsPosessesBlockt? :type Boolean))
  (Utilities|FlowControl|DoOnce false
    (:Completed
      (Audio|Components|Audio|Play (Variables|Default|GetSC_Holzkiste) 0.0)
      (bind _rotate (Timeline|Timeline PlayFromStart)
        (:Update
          (Transformation|SetRelativeRotation (Variables|Default|GetKistenDeggel) (Math|Rotator|MakeRotator 0.0 (* _rotate -1e+02) 0.0) false false))
        (:Finished
          (Audio|Components|Audio|Stop (Variables|Default|GetSC_Holzkiste)))))))

(fn ConstructionScript
  (|CallParentFunction))