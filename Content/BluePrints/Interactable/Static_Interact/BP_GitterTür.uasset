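; BP_GitterTür is an interactable metal grate door that swings open and closed when the player interacts with it.
; Each InteractPickup plays the metal door sound and uses a FlipFlop to alternate between playing a Timeline forward and in reverse.
; The Timeline scales its Rotate track by Öffnungswinkel to set the yaw of BankGitterTür.
; A DoOnce blocks further interaction until the Timeline finishes.
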(event EventInteractPickup
  (params (PlayerCharacter :type BP%20Player%20Character%20Object%20Reference) (WillPlayerWatchingObjectInHand? :type Boolean) (IsObjectInHand? :type Boolean) (IsPosessesBlockt? :type Boolean))
  (Utilities|FlowControl|DoOnce false :!label _label
    (:Completed
      (Audio|Components|Audio|Play (Variables|Default|GetSC_MetalDoor) 0.0)
      (Utilities|FlowControl|FlipFlop
        (:A
          (bind _rotate (Timeline|Timeline PlayFromStart)
            (:Update
              (Transformation|SetRelativeRotation (Variables|Default|GetBank_GitterTür) (Math|Rotator|MakeRotator 0.0 0.0 (* _rotate (Variables|Default|GetÖffnungswinkel))) false false))
            (:Finished
              (goto _label Reset))))
        (:B
          (Timeline|Timeline ReverseFromEnd))))))

(fn ConstructionScript
  (|CallParentFunction))