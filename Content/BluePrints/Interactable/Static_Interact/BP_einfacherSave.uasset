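; Simple interactable safe whose hinged door swings open or closed on alternate InteractPickup calls.
; Each accepted interaction plays the metal door sound, and a FlipFlop runs a timeline forward or in reverse to yaw the active hinge up to 125 degrees, blocking input until it finishes.
; The construction script uses RotateLeft to attach the door to the left or right side and show only that side's hinge meshes.
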(event EventInteractPickup
  (params (PlayerCharacter :type BP%20Player%20Character%20Object%20Reference) (WillPlayerWatchingObjectInHand? :type Boolean) (IsObjectInHand? :type Boolean) (IsPosessesBlockt? :type Boolean))
  (if (not (Variables|Default|GetInputBlockIsOn))
    (Audio|Components|Audio|Play (Variables|Default|GetSC_MetalDoor) 0.0)
    (Utilities|FlowControl|FlipFlop
      (:A
        (bind _newtrack_0 (Timeline|Timeline PlayFromStart)
          (:Update
            (Variables|Default|SetInputBlockIsOn true)
            (Transformation|SetRelativeRotation (select (Variables|Default|GetRotate%20Left) (Variables|Default|GetTürschanir_L) (Variables|Default|GetTürschanir_R)) (Math|Rotator|MakeRotator 0.0 0.0 (* (* _newtrack_0 125.0) (Math|Float|SelectFloat 1.0 -1.0 (Variables|Default|GetRotate%20Left)))) false false))
          (:Finished
            (Variables|Default|SetInputBlockIsOn false))))
      (:B
        (Timeline|Timeline ReverseFromEnd)))))

(fn ConstructionScript
  (|CallParentFunction)
  (Transformation|AttachComponentToComponent (Variables|Default|GetTresorTürBase) (select (Variables|Default|GetRotate%20Left) (Variables|Default|GetL) (Variables|Default|GetR)) "None" "SnapToTarget" "SnapToTarget" "KeepRelative" true)
  (if (Variables|Default|GetRotate%20Left)
    (Rendering|SetVisibility (Variables|Default|GetTürschanir_L) true false)
    (Rendering|SetVisibility (Variables|Default|GetTürschanir_R) false false)
    (else
      (Rendering|SetVisibility (Variables|Default|GetTürschanir_L) false false)
      (Rendering|SetVisibility (Variables|Default|GetTürschanir_R) true false))))