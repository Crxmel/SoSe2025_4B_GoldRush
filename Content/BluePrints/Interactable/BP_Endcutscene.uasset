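; BP_Endcutscene is an interactable actor that starts a level sequence, presumably the ending cutscene, once its process finishes.
; GetProsses calls the parent logic, waits one second beyond SmoothProsessDuration, then plays the sequence player of the NewVar reference.
; A separate AufzugTrigger (elevator trigger) event instantly shifts the root component 1000 units upward.
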(event Custom|AufzugTrigger
  (Class|SceneComponent|AddWorldTransform (Variables|Default|GetDefaultSceneRoot) (Math|Transform|MakeTransform "0.000000,0.000000,1000.000000" "0, 0, 0" "1.000000,1.000000,1.000000") false false))

(event EventBeginPlay)

(event Collision|EventActorBeginOverlap
  (params (OtherActor :type Actor%20Object%20Reference)))

(event EventTick
  (params (DeltaSeconds :type Float%20%28single-precision%29)))

(event EventGetProsses
  (|CallParentFunction)
  (Utilities|FlowControl|Delay (+ (Variables|Default|GetSmooth%20Prosess%20Duration) 1.0))
  (Sequencer|Player|Play (Variables|/Script/LevelSequence.LevelSequenceActor|GetSequencePlayer (Variables|Default|GetNewVar)) :!class /Script/MovieScene.MovieSceneSequencePlayer))

(fn ConstructionScript
  (|CallParentFunction))